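; NPC Blueprint that handles a catch attack and a timed stun reaction, and always returns false for item-use interactions.
; Catch plays the attack montage, while Stunned plays a pain scream and flags the stun in NPC_AnimBP.
; Tick counts the stun down by a fixed per-frame step, so its duration is frame-rate dependent.
; AlphaStunned snaps on halfway through, and IsStunned clears when the countdown ends.
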(event `/Game/Content/Blueprints/BPi_Interface.Catch`
  (`|PlayMontage` (`self.Mesh`) "/Game/AI/Animations/NPC_Attacks_Montage.NPC_Attacks_Montage"))

(event `/Game/Content/Blueprints/BPi_Interface.Stunned`
  (set `self.StunnedTimer` 2.6)
  (bind _asnpc_anim_bp (cast `/Game/AI/Animations/NPC_AnimBP` (`SkeletalMeshComponent.GetAnimInstance` (`self.Mesh`))))
  (set `/Game/AI/Animations/NPC_AnimBP.isStunned` true _asnpc_anim_bp)
  (`GameplayStatics.PlaySound2D` "/Game/Content/Audio/Themes/AmbianceSounds/SoundEffect/Scream-death-painM.Scream-death-painM" 1.0 1.0 0.0 null null)
  (set `self.StartStunnedTimer` true))

(event `self.ReceiveTick`
  (params (DeltaSeconds :type "Float (single-precision)"))
  (bind _stunnedtimer (`self.StunnedTimer`))
  (if (`self.StartStunnedTimer`)
    (set `self.StunnedTimer` (- (`self.StunnedTimer`) 0.05))
    (if (<= _stunnedtimer 1.3)
      (set `/Game/AI/Animations/NPC_AnimBP.alphaStunned` 1.0 (stale `/Game/Content/Blueprints/BPi_Interface.Stunned` _asnpc_anim_bp))
      (if (<= _stunnedtimer 0.1)
        (set `self.StartStunnedTimer` false)
        (set `/Game/AI/Animations/NPC_AnimBP.isStunned` false (stale `/Game/Content/Blueprints/BPi_Interface.Stunned` _asnpc_anim_bp)))
      (else
        (set `/Game/AI/Animations/NPC_AnimBP.alphaStunned` 0.0 (stale `/Game/Content/Blueprints/BPi_Interface.Stunned` _asnpc_anim_bp))))))

(fn `Use Item Interact`
  (params (Item :type "/Game/Inventory/InventoryObject Object Reference"))
  (returns (Success :type Boolean))
  (return false))

(fn `UserConstructionScript`)