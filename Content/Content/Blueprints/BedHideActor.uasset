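; Hideable bed actor that lets the player hide underneath it and look around from its own camera.
; Box overlap shows a prompt widget, enables input and opens a gate for Interact; leaving reverses this.
; Interact toggles hiding: character visibility and collision, a blended view-target switch, and the character's IsHiding flag.
; While hidden, look axes accumulate clamped pitch and yaw for MoveCamera; otherwise they pass to the character.
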(event `InputAction|Interact`
  (params (Key :type "Key Structure"))
  (:`Pressed`
    (`/Engine/EditorBlueprintResources/StandardMacros.Gate` true :!label _label
      (:`Exit`
        (`self.Hiding`)
        (`self.MoveCamera`)
        (`KismetSystemLibrary.Delay` 0.2)
        (`self.EnableInput` (`GameplayStatics.GetPlayerController` 0) :!label _label_2)
        (goto _label :!via `Open`)))))

(event `self.Box.OnComponentBeginOverlap`
  (params (OverlappedComponent :type "PrimitiveComponent Object Reference") (OtherActor :type "Actor Object Reference") (OtherComp :type "PrimitiveComponent Object Reference") (OtherBodyIndex :type Integer) (bFromSweep :type Boolean) (SweepResult :type "HitResult Structure (by ref)"))
  (bind _asfpscharacter_bp (cast `/Game/Character/Blueprints/FPSCharacter_BP` OtherActor))
  (bind _returnvalue (`|CreateWidget` "/Game/Content/HUD/Hide_WP.Hide_WP_C"))
  (`UserWidget.AddToViewport` _returnvalue 0)
  (set `self.CharacterRef` _asfpscharacter_bp)
  (goto _label_2))

(event `self.Box.OnComponentEndOverlap`
  (params (OverlappedComponent :type "PrimitiveComponent Object Reference") (OtherActor :type "Actor Object Reference") (OtherComp :type "PrimitiveComponent Object Reference") (OtherBodyIndex :type Integer))
  (cast `/Game/Character/Blueprints/FPSCharacter_BP` OtherActor)
  (`Widget.RemoveFromParent` (stale `self.Box.OnComponentBeginOverlap` _returnvalue))
  (`self.DisableInput` (`GameplayStatics.GetPlayerController` 0) null)
  (goto _label :!via `Close`))

(event `InputAxis|LookUp`
  (params (AxisValue :type "Float (single-precision)"))
  ;[1 1 1] Move camera while under the bed
  (if (`self.IsHiding`)
    (bind _output_get (set `self.Pitch` (`KismetMathLibrary.FClamp` (+ (`self.Pitch`) AxisValue) -50.0 20.0)))
    (else
      (`Pawn.AddControllerPitchInput` (`self.CharacterRef`) AxisValue))))

(event `MoveCamera`
  ;[1 1 1] Move camera while under the bed
  (if (`self.IsHiding`)
    (`SceneComponent.K2_SetRelativeRotation` (`self.Camera`) (`KismetMathLibrary.MakeRotator` 0.0 (* (stale `InputAxis|LookUp` _output_get) -1.0) (* (stale `InputAxis|Turn` _output_get) 1.0)) false false)
    (`KismetSystemLibrary.Delay` 0.001)))

(event `InputAxis|Turn`
  (params (AxisValue :type "Float (single-precision)"))
  ;[1 1 1] Move camera while under the bed
  (if (`self.IsHiding`)
    (bind _output_get (set `self.Yaw` (`KismetMathLibrary.FClamp` (+ (`self.Yaw`) AxisValue) -60.0 60.0)))
    (else
      (`Pawn.AddControllerYawInput` (`self.CharacterRef`) AxisValue))))

(fn `Hiding`
  (bind _returnvalue (`GameplayStatics.GetPlayerController` 0))
  (bind _characterref (`self.CharacterRef`))
  (if (`self.IsHiding`)
    (set `self.IsHiding` false)
    (`self.SetActorHiddenInGame` _characterref false)
    (`self.SetActorEnableCollision` _characterref true)
    (`PlayerController.SetViewTargetWithBlend` _returnvalue null 0.8 "VTBlend_Linear" 0.0 false)
    (else
      (set `self.IsHiding` true)
      (`self.SetActorHiddenInGame` _characterref true)
      (`self.SetActorEnableCollision` _characterref false)
      (`PlayerController.SetViewTargetWithBlend` _returnvalue self 0.8 "VTBlend_Linear" 0.0 false)))
  (bind _asfpscharacter_bp (cast `/Game/Character/Blueprints/FPSCharacter_BP` (`GameplayStatics.GetPlayerCharacter` 0)))
  (set `/Game/Character/Blueprints/FPSCharacter_BP.IsHiding` (`self.IsHiding`) _asfpscharacter_bp))

(fn `UserConstructionScript`)