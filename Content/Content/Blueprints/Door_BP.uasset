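; Interactable door Blueprint that swings open and closed with creak sounds and noise events attributed to the player.
; Interaction switches on a Closed, Opening, Open or Closing state, playing the timeline from start or in reverse from end, or forward from its current position mid-swing.
; The timeline scales the open rotation onto the door mesh, derives the moving state from its direction, and settles it when finished.
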(event `self.ReceiveBeginPlay`
  (`StaticMeshComponent.SetStaticMesh` (`self.Door`) (`self.Mesh`)))

(event `/Game/Content/Blueprints/BPi_Interface.Interaction`
  (params (Interactor :type "Actor Object Reference"))
  (bind _returnvalue (`self.K2_GetActorLocation`))
  (bind _returnvalue_2 (`GameplayStatics.GetPlayerCharacter` 0))
  (bind _maxrange (`self.MaxRange`))
  (bind _loudness (`self.Loudness`))
  (bind _tag (`self.Tag`))
  (switch `/Game/Content/Blueprints/Enums/DoorState` (`self.State`)
    (:`NewEnumerator0`
      ;[1 1 1] Noise Event
      (`GameplayStatics.PlaySoundAtLocation` "/Game/Content/Audio/DoorSound/DoorCreak_Wood_Closing.DoorCreak_Wood_Closing" _returnvalue (struct) 1.0 1.0 0.0 null null null)
      (`AISense_Hearing.ReportNoiseEvent` _returnvalue _loudness _returnvalue_2 _maxrange _tag)
      (bind (_direction _dooropening) (`Timeline|DoorAnimation` :!via `PlayFromStart` :!label _label)
        (:`Update`
          ;[1 1 1] Update the rotation of the door
          (`SceneComponent.K2_SetRelativeRotation` (`self.Door`) (* (`self.OpenDoorRotation`) _dooropening) false false)
          (if (`|EnumEquality` _direction "Forward")
            (set `self.State` "NewEnumerator3")
            (else
              (set `self.State` "NewEnumerator2"))))
        (:`Finished`
          ;[1 1 1] Finished Closing or Openings
          (switch `/Game/Content/Blueprints/Enums/DoorState` (`self.State`)
            (:`NewEnumerator2`
              (set `self.State` "NewEnumerator0"))
            (:`NewEnumerator3`
              (set `self.State` "NewEnumerator1"))))))
    (:`NewEnumerator1`
      (`GameplayStatics.PlaySoundAtLocation` "/Game/Content/Audio/DoorSound/DoorCreak_Wood_Open.DoorCreak_Wood_Open" _returnvalue (struct) 0.5 1.0 0.0 null null null)
      (`AISense_Hearing.ReportNoiseEvent` _returnvalue _loudness _returnvalue_2 _maxrange _tag)
      (goto _label :!via `ReverseFromEnd`))
    (:`NewEnumerator2`
      (`GameplayStatics.PlaySoundAtLocation` "/Game/Content/Audio/DoorSound/DoorCreak_Wood_Closing.DoorCreak_Wood_Closing" _returnvalue (struct) 1.0 1.0 0.0 null null null)
      (`AISense_Hearing.ReportNoiseEvent` _returnvalue _loudness _returnvalue_2 _maxrange _tag :!label _label_2)
      (goto _label))
    (:`NewEnumerator3`
      (`GameplayStatics.PlaySoundAtLocation` "/Game/Content/Audio/DoorSound/DoorCreak_Wood_Open.DoorCreak_Wood_Open" _returnvalue (struct) 0.5 1.0 0.0 null null null)
      (goto _label_2))))

(fn `UserConstructionScript`)