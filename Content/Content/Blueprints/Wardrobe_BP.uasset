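; Possessable wardrobe the player can hide in, with a swinging door pivot and a Hide_WP widget shown inside HideBox.
; openWardrobe alternates opening and closing through a yaw timeline, disabling door collision during motion.
; When FPSCharacter_BP overlaps Box, the controller possesses the wardrobe and the door timeline reverses.
; Interact plays a second door timeline, calling Possess with no pawn specified on each update.
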(event `openWardrobe`
  (`PrimitiveComponent.SetCollisionEnabled` (`self.WardrobeDoor`) "NoCollision")
  (`PrimitiveComponent.SetCollisionEnabled` (`self.WardrobeDoor1`) "NoCollision")
  (`/Engine/EditorBlueprintResources/StandardMacros.FlipFlop`
    (:`A`
      (bind (_direction _newtrack_0) (`Timeline|wardrobeTimeline` :!via `PlayFromStart` :!label _label)
        (:`Update`
          (`SceneComponent.K2_SetRelativeRotation` (`self.Pivot`) (`KismetMathLibrary.MakeRotator` 0.0 0.0 _newtrack_0) false false))
        (:`Finished`
          (`PrimitiveComponent.SetCollisionEnabled` (`self.WardrobeDoor`) "QueryAndPhysics")
          (`PrimitiveComponent.SetCollisionEnabled` (`self.WardrobeDoor1`) "QueryAndPhysics"))))
    (:`B`
      (goto _label :!via `ReverseFromEnd`))))

(event `self.Box.OnComponentBeginOverlap`
  (params (OverlappedComponent :type "PrimitiveComponent Object Reference") (OtherActor :type "Actor Object Reference") (OtherComp :type "PrimitiveComponent Object Reference") (OtherBodyIndex :type Integer) (bFromSweep :type Boolean) (SweepResult :type "HitResult Structure (by ref)"))
  (cast `/Game/Character/Blueprints/FPSCharacter_BP` OtherActor)
  (`Controller.Possess` (`GameplayStatics.GetPlayerController` 0) self)
  (goto _label :!via `ReverseFromEnd`))

(event `InputAction|Interact`
  (params (Key :type "Key Structure"))
  (:`Pressed`
    (`PrimitiveComponent.SetCollisionEnabled` (`self.WardrobeDoor`) "NoCollision")
    (`PrimitiveComponent.SetCollisionEnabled` (`self.WardrobeDoor1`) "NoCollision")
    (bind (_direction _newtrack_0) (`Timeline|Timeline_0` :!via `PlayFromStart`)
      (:`Update`
        (`SceneComponent.K2_SetRelativeRotation` (`self.Pivot`) (`KismetMathLibrary.MakeRotator` 0.0 0.0 _newtrack_0) false false)
        (`Controller.Possess` (`GameplayStatics.GetPlayerController` 0) null))
      (:`Finished`
        (`PrimitiveComponent.SetCollisionEnabled` (`self.WardrobeDoor`) "QueryAndPhysics")
        (`PrimitiveComponent.SetCollisionEnabled` (`self.WardrobeDoor1`) "QueryAndPhysics")))))

(event `self.HideBox.OnComponentBeginOverlap`
  (params (OverlappedComponent :type "PrimitiveComponent Object Reference") (OtherActor :type "Actor Object Reference") (OtherComp :type "PrimitiveComponent Object Reference") (OtherBodyIndex :type Integer) (bFromSweep :type Boolean) (SweepResult :type "HitResult Structure (by ref)"))
  (bind _returnvalue (`|CreateWidget` "/Game/Content/HUD/Hide_WP.Hide_WP_C"))
  (`UserWidget.AddToViewport` _returnvalue 0))

(event `self.HideBox.OnComponentEndOverlap`
  (params (OverlappedComponent :type "PrimitiveComponent Object Reference") (OtherActor :type "Actor Object Reference") (OtherComp :type "PrimitiveComponent Object Reference") (OtherBodyIndex :type Integer))
  (`Widget.RemoveFromParent` (stale `self.HideBox.OnComponentBeginOverlap` _returnvalue)))

(fn `UserConstructionScript`)