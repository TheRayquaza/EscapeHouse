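; Door receiver actor that rotates by a wanted offset from its starting rotation when its event r fires.
; A timeline multiplier scales that offset on each axis, added to the rotation cached at BeginPlay.
; With OneTimeReceiver set, the first trigger clears the flag, plays a spatialized creak and runs the timeline forward.
; Triggers with the flag unset alternate forward and reverse playback through a FlipFlop, without sound.
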(event `self.ReceiveBeginPlay`
  (`parent.ReceiveBeginPlay`)
  (set `self.InitialRotation` (`self.K2_GetActorRotation` self)))

(event `self.Receiver`
  (if (`self.OneTimeReceiver`)
    (set `self.OneTimeReceiver` false)
    (`GameplayStatics.PlaySoundAtLocation` "/Game/Content/Audio/Sounds/Spatialized/ObjectSounds/Door/Normal/DoorCreak_Wood_Open.DoorCreak_Wood_Open" (`self.K2_GetActorLocation`) (struct) 2.0 0.75 0.0 "/Game/Content/Audio/Attenuation/SpatializedSounds.SpatializedSounds" null null)
    (bind (_direction _multiplyer) (`Timeline|Animation` :!via `PlayFromStart` :!label _label)
      (:`Update`
        (`self.K2_SetActorRotation` (`KismetMathLibrary.MakeRotator` (+ (.roll (`self.InitialRotation`)) (* (.roll (`self.WantedRotation`)) _multiplyer)) (+ (.pitch (`self.InitialRotation`)) (* (.pitch (`self.WantedRotation`)) _multiplyer)) (+ (.yaw (`self.InitialRotation`)) (* (.yaw (`self.WantedRotation`)) _multiplyer))))))
    (else
      (`/Engine/EditorBlueprintResources/StandardMacros.FlipFlop`
        (:`A`
          (goto _label :!via `PlayFromStart`))
        (:`B`
          (goto _label :!via `ReverseFromEnd`))))))

(fn `UserConstructionScript`
  (`parent.UserConstructionScript`))