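; CageWire receiver actor that slides between its start position and a relative target offset when its `r` event fires.
; A timeline multiplier scales the offset from the location saved at BeginPlay, playing Close forward and Open in reverse.
; A FlipFlop alternates the directions, but with OneTimeReceiver set, the first trigger only clears that flag and plays forward, so later triggers still reach the FlipFlop.
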(event `self.ReceiveBeginPlay`
  (`parent.ReceiveBeginPlay`)
  (set `self.InitialLocation` (`self.K2_GetActorLocation` self)))

(event `self.Receiver`
  (if (`self.OneTimeReceiver`)
    (set `self.OneTimeReceiver` false)
    (`AudioComponent.Play` (`self.Close`) 0.0 :!label _label)
    (bind (_direction _multiplier) (`Timeline|Animation` :!via `PlayFromStart` :!label _label_2)
      (:`Update`
        (`self.K2_SetActorLocation` (`KismetMathLibrary.MakeVector` (+ (.x (`self.InitialLocation`)) (* _multiplier (.x (`self.RelativeWantedLocation`)))) (+ (.y (`self.InitialLocation`)) (* _multiplier (.y (`self.RelativeWantedLocation`)))) (+ (.z (`self.InitialLocation`)) (* _multiplier (.z (`self.RelativeWantedLocation`))))))))
    (else
      (`/Engine/EditorBlueprintResources/StandardMacros.FlipFlop`
        (:`A`
          (goto _label))
        (:`B`
          (`AudioComponent.Play` (`self.Open`) 0.0)
          (goto _label_2 :!via `ReverseFromEnd`))))))

(fn `UserConstructionScript`
  (`parent.UserConstructionScript`))