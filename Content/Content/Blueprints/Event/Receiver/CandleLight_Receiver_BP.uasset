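; Candle light receiver actor that lights up when its custom event r is called from outside the graph.
; The event shows the point light and spawns a small, scaled-down particle system component above the actor's origin.
; A Brightness timeline then drives the light's intensity through a scaled multiplier curve.
; The graph has no logic to put the candle out or guard against repeated calls.
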(event `self.Receiver`
  (`SceneComponent.SetVisibility` (`self.PointLight`) true false)
  (`AddComponent|NODE_AddParticleSystemComponent-0` :`RelativeTransform` (`KismetMathLibrary.MakeTransform` (0.0 0.0 58.0) (struct) (0.25 0.25 0.25)))
  (bind (_direction _multiplier) (`Timeline|Brightness`)
    (:`Update`
      (`LightComponent.SetIntensity` (`self.PointLight`) (* _multiplier 400.0)))))

(fn `UserConstructionScript`
  (`parent.UserConstructionScript`))