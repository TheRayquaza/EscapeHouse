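; Receiver actor for a wooden plank that falls when triggered.
; Its custom event `r` turns on physics simulation for the static mesh and plays a falling-plank sound at the actor's location.
; After a short fixed delay it turns physics off again, so the fall is limited by time rather than by landing detection.
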(event `self.Receiver`
  (`PrimitiveComponent.SetSimulatePhysics` (`self.StaticMeshComponent`) true)
  (`GameplayStatics.PlaySoundAtLocation` "/Game/Content/Audio/Sounds/Spatialized/ObjectSounds/Plank/PlankFalling.PlankFalling" (`self.K2_GetActorLocation`) (struct) 1.0 1.0 0.0 null null null)
  (`KismetSystemLibrary.Delay` 0.6)
  (`PrimitiveComponent.SetSimulatePhysics` (`self.StaticMeshComponent`) false))

(fn `UserConstructionScript`
  (`parent.UserConstructionScript`))