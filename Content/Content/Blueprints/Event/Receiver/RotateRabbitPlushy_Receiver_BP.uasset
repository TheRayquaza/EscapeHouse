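; Event receiver Blueprint that rotates its actor, by name a rabbit plushy, when its receiver event fires.
; It stores the starting rotation on BeginPlay and uses a one-time flag so the rotation runs only once.
; A timeline multiplier scales the wanted rotation offset, which is added per axis to the starting rotation on each update.
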(event `self.ReceiveBeginPlay`
  (`parent.ReceiveBeginPlay`)
  (set `self.InitialRotation` (`self.K2_GetActorRotation` self)))

(event `self.Receiver`
  (if (`self.OneTimeReceiver`)
    (set `self.OneTimeReceiver` false)
    (bind (_direction _multiplyer) (`Timeline|Animation` :!via `PlayFromStart`)
      (:`Update`
        (`self.K2_SetActorRotation` (`KismetMathLibrary.MakeRotator` (+ (.roll (`self.InitialRotation`)) (* (.roll (`self.WantedRotation`)) _multiplyer)) (+ (.pitch (`self.InitialRotation`)) (* (.pitch (`self.WantedRotation`)) _multiplyer)) (+ (.yaw (`self.InitialRotation`)) (* (.yaw (`self.WantedRotation`)) _multiplyer))))))))

(fn `UserConstructionScript`
  (`parent.UserConstructionScript`))