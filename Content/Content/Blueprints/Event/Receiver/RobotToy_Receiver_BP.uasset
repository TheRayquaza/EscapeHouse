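; RobotToy_Receiver_BP is a robot toy receiver Blueprint that gives a timed light and sound response when triggered.
; Its custom event `r` plays WaveAudio and shows two point lights, then hides both lights after a short delay.
; BeginPlay, overlap and Tick are unused, so the response depends on `r` being called, and nothing in this Blueprint calls it.
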(event `self.Receiver`
  (`AudioComponent.Play` (`self.WaveAudio`) 0.0)
  (`SceneComponent.SetVisibility` (`self.PointLight`) true false)
  (`SceneComponent.SetVisibility` (`self.PointLight1`) true false)
  (`KismetSystemLibrary.Delay` 3.0)
  (`SceneComponent.SetVisibility` (`self.PointLight`) false false)
  (`SceneComponent.SetVisibility` (`self.PointLight1`) false false))

(fn `UserConstructionScript`
  (`parent.UserConstructionScript`))