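; Secret door receiver that moves and rotates the door from its starting pose when triggered.
; It records its initial location and rotation at BeginPlay.
; Its `r` event, gated by OneTimeReceiver, plays the DoorFalls timeline from the start, whose Multiplier track scales the WantedLocation and WantedRotation offsets added to that pose.
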(event `self.ReceiveBeginPlay`
  (`parent.ReceiveBeginPlay`)
  (set `self.InitialLocation` (`self.K2_GetActorLocation` self))
  (set `self.InitialRotation` (`self.K2_GetActorRotation` self)))

(event `self.Receiver`
  (if (`self.OneTimeReceiver`)
    (bind (_direction _multiplier) (`Timeline|DoorFalls` :!via `PlayFromStart`)
      (:`Update`
        (`self.K2_SetActorLocationAndRotation` (+ (`self.InitialLocation`) (`KismetMathLibrary.MakeVector` (* _multiplier (.x (`self.WantedLocation`))) (* _multiplier (.y (`self.WantedLocation`))) (* _multiplier (.z (`self.WantedLocation`))))) (`KismetMathLibrary.MakeRotator` (+ (* (.roll (`self.WantedRotation`)) _multiplier) (.roll (`self.InitialRotation`))) (+ (* (.pitch (`self.WantedRotation`)) _multiplier) (.pitch (`self.InitialRotation`))) (+ (* (.yaw (`self.WantedRotation`)) _multiplier) (.yaw (`self.InitialRotation`)))))))))

(fn `UserConstructionScript`
  (`parent.UserConstructionScript`))