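; Secret book interactable that acts as an event sender, tilting when used to trigger linked receiver actors.
; Interaction plays a sound and the Use timeline, which rotates the book from its initial rotation by a scaled WantedRotation offset.
; When the timeline finishes, it calls Receiver on every linked actor and plays the shelf mechanism sound.
; The first path is gated by a one-time flag, while later interactions decrement a use counter to play the timeline again.
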(event `self.ReceiveBeginPlay`
  (`parent.ReceiveBeginPlay`)
  (set `self.InitialRotation` (`self.K2_GetActorRotation` self)))

(event `/Game/Content/Blueprints/BPi_Interface.Interaction`
  (params (Interactor :type "Actor Object Reference"))
  (bind _numbersender (`self.NumberSender`))
  (if (`self.OneTimeSender`)
    (set `self.OneTimeSender` false)
    (`AudioComponent.Play` (`self.SpecialBookMechanism`) 0.0)
    (bind (_direction _multiply) (`Timeline|Use` :!label _label)
      (:`Update`
        (`self.K2_SetActorRotation` (`KismetMathLibrary.MakeRotator` (+ (.roll (`self.InitialRotation`)) (* (.roll (`self.WantedRotation`)) _multiply)) (+ (.pitch (`self.InitialRotation`)) (* (.pitch (`self.WantedRotation`)) _multiply)) (+ (.yaw (`self.InitialRotation`)) (* (.yaw (`self.WantedRotation`)) _multiply)))))
      (:`Finished`
        (for _array_element (`self.ReceiverActorS`)
          (`/Game/Content/Blueprints/Event/Receiver/BasicReceiver_BP.Receiver` _array_element))
        (`AudioComponent.Play` (`self.ShelfMechanismEvent`) 0.0)))
    (elif (not (== _numbersender 0))
      (`/Engine/EditorBlueprintResources/StandardMacros.DecrementInt` _numbersender
        (:`  `
          (goto _label))))))

(fn `UserConstructionScript`
  (`parent.UserConstructionScript`))