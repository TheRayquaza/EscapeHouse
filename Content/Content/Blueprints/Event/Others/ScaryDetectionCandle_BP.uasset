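; ScaryDetectionCandle_BP is a candle that lights itself when the player comes within a detection distance.
; Each tick it measures the distance from the player character to itself and compares it with DistanceDetection.
; On first detection, a DoOnce makes the point light visible, adds a small particle system slightly above the origin, and disables ticking, so it never switches back off.
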(event `self.ReceiveTick`
  (params (DeltaSeconds :type "Float (single-precision)"))
  (if (<= (`KismetMathLibrary.Vector_Distance` (`self.K2_GetActorLocation` (`GameplayStatics.GetPlayerCharacter` 0)) (`self.K2_GetActorLocation` self)) (`self.DistanceDetection`))
    (`/Engine/EditorBlueprintResources/StandardMacros.DoOnce` false
      (:`Completed`
        (`SceneComponent.SetVisibility` (`self.PointLight`) true false)
        (`AddComponent|NODE_AddParticleSystemComponent-0` :`RelativeTransform` (`KismetMathLibrary.MakeTransform` (0.0 0.0 17.0) (struct) (0.25 0.25 0.25)))
        (`self.SetActorTickEnabled` false)))))

(fn `UserConstructionScript`)