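; Trigger box event that plays sounds when actors of allowed classes enter or leave it.
; On begin overlap it can set the player character's ambiance sound Configuration parameter, before any class filtering.
; Exact class matches play the begin sound only while OneTimeEvent is true, which is then cleared, so it fires at most once.
; The end-overlap sound plays on every matching exit.
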(event `self.ReceiveActorBeginOverlap`
  (params (OtherActor :type "Actor Object Reference"))
  (if (`self.ChangeLevelAmbiance`)
    (bind _asfpscharacter_child_bp (cast `/Game/Character/ChildCharacter/FPSCharacterChild_BP` (`GameplayStatics.GetPlayerCharacter` 0)))
    (`AudioComponent.SetIntParameter` (`/Game/Character/ChildCharacter/FPSCharacterChild_BP.AmbianceSound` _asfpscharacter_child_bp) "Configuration" (`self.AmbianceConfiguration`)))
  (for _array_element (`self.AllowedClass`)
    (if (== _array_element (`GameplayStatics.GetObjectClass` OtherActor))
      (if (`self.OneTimeEvent`)
        (set `self.OneTimeEvent` false)
        (`AudioComponent.Play` (`self.B_OverlapSound`) 0.0)))))

(event `self.ReceiveActorEndOverlap`
  (params (OtherActor :type "Actor Object Reference"))
  (for _array_element (`self.AllowedClass`)
    (if (== _array_element (`GameplayStatics.GetObjectClass` OtherActor))
      (`AudioComponent.Play` (`self.E_OverlapSound`) 0.0))))

(fn `UserConstructionScript`)