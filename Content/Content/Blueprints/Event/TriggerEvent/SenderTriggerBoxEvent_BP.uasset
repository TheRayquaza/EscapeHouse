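; One-shot trigger box that fires linked event actors and ambiance audio when an actor overlaps it.
; The first overlap clears OneTimeSender, even if the actor's class is not in OverlappedCharacterClasses.
; On an exact class match, it calls Receiver on receiver actors and switches on class display name to activate sender actors.
; If Audio is set, it plays it and sets the FPS character's AmbianceSound configuration parameter.
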(event `self.ReceiveActorBeginOverlap`
  (params (OtherActor :type "Actor Object Reference"))
  (bind _audio (`self.Audio`))
  (if (`self.OneTimeSender`)
    (set `self.OneTimeSender` false)
    (for _array_element (`self.OverlappedCharacterClasses`)
      (if (== _array_element (`GameplayStatics.GetObjectClass` OtherActor))
        ;[1 1 1] Basic Function
        (for _array_element_2 (`self.ReceiverActorS`)
          (`/Game/Content/Blueprints/Event/Receiver/BasicReceiver_BP.Receiver` _array_element_2))
        ;[1 1 1] Specific for Sender Actors which need activations or something else
        (for _array_element_3 (`self.SenderActorS`)
          (switch `string` (`KismetSystemLibrary.GetClassDisplayName` (`GameplayStatics.GetObjectClass` _array_element_3))
            (:`Button_Sender_BP_C`
              (set `/Game/Content/Blueprints/Event/Sender/BasicSender_BP.IsActivated` true _array_element_3))))
        ;[1 1 1] SoundAmbiance
        (if (!= _audio null)
          (`AudioComponent.Play` _audio 0.0)
          (bind _asfpscharacter_child_bp (cast `/Game/Character/ChildCharacter/FPSCharacterChild_BP` OtherActor))
          (`AudioComponent.SetIntParameter` (`/Game/Character/ChildCharacter/FPSCharacterChild_BP.AmbianceSound` _asfpscharacter_child_bp) "Configuration" (`self.AmbianceConfiguration`)))))))

(fn `UserConstructionScript`)