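; Configurable point light that can buzz and play a "creepy" intensity animation.
; The construction script applies brightness and color, and sets the buzz sound volume from IsBuzzing.
; When CreepyLight is set, a timeline drives light intensity from BeginPlay.
; SwitchLight toggles the light, stopping the timeline when off and replaying it after a short delay when on.
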(event `self.ReceiveBeginPlay`
  (if (`self.CreepyLight`) :!label _label
    (bind (_direction _intensity) (`Timeline|CreepyLightAnimation` :!via `PlayFromStart`)
      (:`Update`
        (`LightComponent.SetIntensity` (`self.LightComponent`) _intensity)))))

(event `Restart Animation`
  (`KismetSystemLibrary.Delay` 3.0)
  (goto _label))

(fn `SwitchLight`
  (params (Boolean :type Boolean))
  (bind _pointlightcomponent (`self.PointLightComponent`))
  (if Boolean
    (`LightComponent.SetIntensity` _pointlightcomponent (`self.Brightness`))
    (`self.Restart Animation`)
    (else
      (`LightComponent.SetIntensity` _pointlightcomponent 0.0)
      (`TimelineComponent.Stop` (`self.CreepyLightAnimation`)))))

(fn `UserConstructionScript`
  (bind _pointlightcomponent (`self.PointLightComponent`))
  (bind _lightsound (`self.LightSound`))
  (`LightComponent.SetIntensity` _pointlightcomponent (`self.Brightness`))
  (`LightComponent.SetLightColor` _pointlightcomponent (`self.Color`) true)
  (if (`self.IsBuzzing`)
    (`AudioComponent.SetVolumeMultiplier` _lightsound 2.0)
    (else
      (`AudioComponent.SetVolumeMultiplier` _lightsound 0.0))))