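; BasicLight_BP is a configurable light that pairs a light component with an optional static mesh.
; The construction script applies the exposed brightness, color and source radius to the light, then assigns the mesh if one is set, repositioning it for the ceiling lamp mesh.
; SwitchLight turns the light on or off by setting its intensity to the configured brightness or to zero.
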(fn `SwitchLight`
  (params (Boolean :type Boolean))
  (bind _light (`self.Light`))
  (if Boolean
    (`LightComponent.SetIntensity` _light (`self.Brightness`))
    (else
      (`LightComponent.SetIntensity` _light 0.0))))

(fn `UserConstructionScript`
  (bind _light (`self.Light`))
  (bind _mesh (`self.Mesh`))
  (`LightComponent.SetIntensity` _light (`self.Brightness`))
  (`LightComponent.SetLightColor` _light (`self.Color`) true)
  (`PointLightComponent.SetSourceRadius` _light (`self.Source Radius`))
  (if (!= (`self.Mesh`) null)
    (`StaticMeshComponent.SetStaticMesh` (`self.StaticMesh`) _mesh)
    (if (== _mesh "/Game/Content/Props/SM_Lamp_Ceiling.SM_Lamp_Ceiling")
      (`SceneComponent.K2_SetRelativeLocationAndRotation` :`self` (`self.StaticMesh`) :`NewLocation` (0.0 0.0 132.0)))))