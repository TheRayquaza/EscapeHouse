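; Removable plank interactable that registers with the player character and inventory when overlapped, showing a prompt and item-specific text.
; Using an item on it sets IsDestroyed, hides the global text, enables mesh physics, then destroys the actor after a timed delay.
; UseItemInteract runs this removal unconditionally; its crowbar and not-destroyed check only feeds the return value, after the flag is set.
; The construction script applies configurable scale and an optional mesh.
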(event `self.ReceiveBeginPlay`
  ;[1 0 0] References
  (bind _asfpscharacter_bp (cast `/Game/Character/Blueprints/FPSCharacter_BP` (`GameplayStatics.GetPlayerCharacter` 0)))
  (set `self.CharacterRef` _asfpscharacter_bp)
  (`PrimitiveComponent.SetSimulatePhysics` (`self.PlankMesh`) false))

(event `self.Box.OnComponentBeginOverlap`
  (params (OverlappedComponent :type "PrimitiveComponent Object Reference") (OtherActor :type "Actor Object Reference") (OtherComp :type "PrimitiveComponent Object Reference") (OtherBodyIndex :type Integer) (bFromSweep :type Boolean) (SweepResult :type "HitResult Structure (by ref)"))
  (bind _inventorycontrollerreference (`/Game/Character/Blueprints/FPSCharacter_BP.InventoryControllerReference` (`self.CharacterRef`)))
  ;[0 0 1] Overlap
  (if (not (`self.IsDestroyed`))
    (`/Game/Character/Blueprints/FPSCharacter_BP.CharacterOverlapsObjects` (`self.CharacterRef`) OtherComp OtherActor self true "This plank can be removed")
    (set `self.IsOverlapped` true)
    (`/Game/Inventory/InventoryController.Set Special Text` _inventorycontrollerreference (`|GetArrayItem` (`/Game/Inventory/InventoryController.Slots` _inventorycontrollerreference) (`/Game/Inventory/InventoryController.ActualSlot` _inventorycontrollerreference)) self)))

(event `self.Box.OnComponentEndOverlap`
  (params (OverlappedComponent :type "PrimitiveComponent Object Reference") (OtherActor :type "Actor Object Reference") (OtherComp :type "PrimitiveComponent Object Reference") (OtherBodyIndex :type Integer))
  ;[0 0 1] Overlap
  (if (`self.IsDestroyed`)
    _
    (else
      _))
  (`/Game/Character/Blueprints/FPSCharacter_BP.CharacterOverlapsObjects` (`self.CharacterRef`) OtherComp OtherActor self false "This plank can be removed")
  (set `self.IsOverlapped` false)
  (`/Game/Inventory/InventoryController.Set Special Text` (`/Game/Character/Blueprints/FPSCharacter_BP.InventoryControllerReference` (`self.CharacterRef`)) null self))

(event `DelayDestroyActor`
  ;[0 1 0.0832] Destroy Actor Event
  (`/Game/Content/HUD/WP_Interface.ShowOrHideGlobalText` (`/Game/Character/Blueprints/FPSCharacter_BP.GlobalWpReference` (`self.CharacterRef`)) false "")
  (`PrimitiveComponent.SetSimulatePhysics` (`self.PlankMesh`) true)
  (`KismetSystemLibrary.Delay` (`self.Timer`))
  (`self.K2_DestroyActor`)
  (set `/Game/Inventory/InventoryController.ActorSelected` null (`/Game/Character/Blueprints/FPSCharacter_BP.InventoryControllerReference` (`self.CharacterRef`))))

(event `/Game/Content/Blueprints/BPi_Interface.ItemsHaveChanged`
  (params (Item :type "/Game/Inventory/InventoryObject Object Reference"))
  ;[0 0.6483 1] Items Have Changed
  (`/Game/Inventory/InventoryController.Set Special Text` (`/Game/Character/Blueprints/FPSCharacter_BP.InventoryControllerReference` (`self.CharacterRef`)) Item self))

(fn `Use Item Interact`
  (params (Item :type "/Game/Inventory/InventoryObject Object Reference"))
  (returns (Success :type Boolean))
  (set `self.IsDestroyed` true)
  (`self.DelayDestroyActor`)
  (return (and (== (`/Game/Inventory/InventoryObject.Type` Item) 1) (not (`self.IsDestroyed`)))))

(fn `UserConstructionScript`
  (bind _mesh (`self.Mesh`))
  (`SceneComponent.SetWorldScale3D` (`self.PlankMesh`) (`self.VectorScale`))
  (if (!= _mesh null)
    (`StaticMeshComponent.SetStaticMesh` (`self.PlankMesh`) _mesh)))