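; Furniture Blueprint with doors that toggle open and closed when the Interact input is pressed.
; OpenDoor disables collision on both door meshes, then a FlipFlop plays the Opening timeline forward or in reverse to drive Pivot1's yaw.
; Collision is restored when the timeline finishes.
; The box overlap only casts to FPSCharacter_BP with no further action, so it does not gate the interaction.
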(event `OpenDoor`
  (`PrimitiveComponent.SetCollisionEnabled` (`self.Doorleft`) "NoCollision")
  (`PrimitiveComponent.SetCollisionEnabled` (`self.DoorRight`) "NoCollision")
  (`/Engine/EditorBlueprintResources/StandardMacros.FlipFlop`
    (:`A`
      (bind (_direction _newtrack_0) (`Timeline|opening` :!via `PlayFromStart` :!label _label)
        (:`Update`
          (`|ExecutionSequence`
            (:`then_0`
              (`SceneComponent.K2_SetRelativeRotation` (`self.Pivot1`) (`KismetMathLibrary.MakeRotator` 0.0 0.0 _newtrack_0) false false))))
        (:`Finished`
          (`PrimitiveComponent.SetCollisionEnabled` (`self.Doorleft`) "QueryAndPhysics")
          (`PrimitiveComponent.SetCollisionEnabled` (`self.DoorRight`) "QueryAndPhysics"))))
    (:`B`
      (goto _label :!via `ReverseFromEnd`))))

(event `self.Box.OnComponentBeginOverlap`
  (params (OverlappedComponent :type "PrimitiveComponent Object Reference") (OtherActor :type "Actor Object Reference") (OtherComp :type "PrimitiveComponent Object Reference") (OtherBodyIndex :type Integer) (bFromSweep :type Boolean) (SweepResult :type "HitResult Structure (by ref)"))
  (cast `/Game/Character/Blueprints/FPSCharacter_BP` OtherActor))

(event `InputAction|Interact`
  (params (Key :type "Key Structure"))
  (:`Pressed`
    (`self.OpenDoor`)))

(fn `UserConstructionScript`)