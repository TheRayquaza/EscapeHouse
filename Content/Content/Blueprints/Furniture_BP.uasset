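; Interactive furniture with two hinged doors that the player opens and closes through an interaction.
; Interaction runs a FlipFlop that plays or reverses a timeline, rotating two pivots in opposite yaw with door collision disabled during the motion.
; A box overlap sends the prompt text to the cached FPS character, setting the overlap flag only on entry while the doors are closed.
; Item use on the furniture always returns false.
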(event `self.ReceiveBeginPlay`
  ;[1 0 0] References
  (bind _asfpscharacter_bp (cast `/Game/Character/Blueprints/FPSCharacter_BP` (`GameplayStatics.GetPlayerCharacter` 0)))
  (set `self.CharacterRef` _asfpscharacter_bp))

(event `OpenDoors`
  ;[1 0 0.4295] Open Doors
  (`PrimitiveComponent.SetCollisionEnabled` (`self.Doorleft`) "NoCollision")
  (`PrimitiveComponent.SetCollisionEnabled` (`self.DoorRight`) "NoCollision")
  (`/Engine/EditorBlueprintResources/StandardMacros.FlipFlop`
    (:`A`
      (set `self.IsOpen` true)
      (bind (_direction _rotation) (`Timeline|opening` :!via `PlayFromStart` :!label _label)
        (:`Update`
          (`SceneComponent.K2_SetRelativeRotation` (`self.Pivot1`) (`KismetMathLibrary.MakeRotator` 0.0 0.0 _rotation) false false)
          (`SceneComponent.K2_SetRelativeRotation` (`self.Pivot2`) (`KismetMathLibrary.MakeRotator` 0.0 0.0 (- 0.0 _rotation)) false false))
        (:`Finished`
          (`PrimitiveComponent.SetCollisionEnabled` (`self.Doorleft`) "QueryAndPhysics")
          (`PrimitiveComponent.SetCollisionEnabled` (`self.DoorRight`) "QueryAndPhysics"))))
    (:`B`
      (set `self.IsOpen` false)
      (goto _label :!via `ReverseFromEnd`))))

(event `self.Box.OnComponentBeginOverlap`
  (params (OverlappedComponent :type "PrimitiveComponent Object Reference") (OtherActor :type "Actor Object Reference") (OtherComp :type "PrimitiveComponent Object Reference") (OtherBodyIndex :type Integer) (bFromSweep :type Boolean) (SweepResult :type "HitResult Structure (by ref)"))
  (bind _characterref (`self.CharacterRef`))
  ;[0 0.8477 1] Overlap
  (if (`self.IsOpen`)
    (`/Game/Character/Blueprints/FPSCharacter_BP.Character Overlaps Objects` _characterref (stale `self.Box.OnComponentEndOverlap` OtherComp) (stale `self.Box.OnComponentEndOverlap` OtherActor) self false "Press F to open/close the furniture" false :!label _label_2)
    (else
      (`/Game/Character/Blueprints/FPSCharacter_BP.Character Overlaps Objects` _characterref OtherComp OtherActor self true "Press F to open/close the furniture" false))))

(event `self.Box.OnComponentEndOverlap`
  (params (OverlappedComponent :type "PrimitiveComponent Object Reference") (OtherActor :type "Actor Object Reference") (OtherComp :type "PrimitiveComponent Object Reference") (OtherBodyIndex :type Integer))
  ;[0 0.8477 1] Overlap
  (if (`self.IsOpen`)
    (goto _label_2)
    (else
      (goto _label_2))))

(event `/Game/Content/Blueprints/BPi_Interface.Interaction`
  (params (Interactor :type "Actor Object Reference"))
  (`self.OpenDoors`))

(fn `Use Item Interact`
  (params (Item :type "/Game/Inventory/InventoryObject Object Reference"))
  (returns (Success :type Boolean))
  (return false))

(fn `UserConstructionScript`)