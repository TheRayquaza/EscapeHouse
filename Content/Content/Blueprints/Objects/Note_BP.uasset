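; Readable note object that shows its text in a WB_ShowNote widget when the player interacts with it.
; Construction script applies a style preset (Mad, Drawing, Letter, Clue) for font, color and paper material, then skins and scales the plane.
; Interaction toggles an active flag, creating and styling the widget on activation but only clearing the flag on deactivation.
; Prompt functions return a fixed "Press F" hint, and item use always returns false.
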(event `self.ReceiveBeginPlay`
  ;[1 0 0] References
  (bind _asfpscharacter_bp (cast `/Game/Character/Blueprints/FPSCharacter_BP` (`GameplayStatics.GetPlayerCharacter` 0)))
  (set `self.CharacterRef` _asfpscharacter_bp))

(event `/Game/Content/Blueprints/BPi_Interface.Interaction`
  (params (Interactor :type "Actor Object Reference"))
  ;[1 0.5 0] Interaction
  (if (`self.IsNoteActive`)
    (set `self.IsNoteActive` false)
    (else
      (set `self.IsNoteActive` true)
      (bind _returnvalue (`|CreateWidget` "/Game/Content/HUD/WB_ShowNote.WB_ShowNote_C"))
      (`UserWidget.AddToViewport` _returnvalue 0)
      (set `/Game/Content/HUD/WB_ShowNote.Text Body` (`self.Note Bodies`) _returnvalue)
      (`self.SetHUDParameters` _returnvalue))))

(fn `Auto Choose Default Text WP`
  (returns (GlobalText :type Text) (SpecificText :type Text) (GlobalShow :type Boolean) (SpecificShow :type Boolean))
  (return "Press F to see the note" "" true false))

(fn `Auto Choose Text WP`
  (params (item :type "/Game/Inventory/InventoryObject Object Reference"))
  (returns (GlobalText :type Text) (SpecificText :type Text) (GlobalShow :type Boolean) (SpecificShow :type Boolean))
  (return "Press F to see the note" "" true false))

(fn `SetHUDParameters`
  (params (HUD :type "/Game/Content/HUD/WB_ShowNote Object Reference"))
  (bind _notebody (`/Game/Content/HUD/WB_ShowNote.NoteBody` HUD))
  (`TextBlock.SetText` _notebody (`|GetArrayItem` (`self.Note Bodies`)))
  (`TextBlock.SetFont` _notebody (make `SlateFontInfo` (`self.FontFamily`) null (struct :`OutlineColor` (struct :`A` 1.0)) "None" (`self.FontSize`)))
  (`TextBlock.SetColorAndOpacity` _notebody (`self.Color`)))

(fn `SetPreset`
  (if (`|EnumInequality` (`self.PresetNote`) "NewEnumerator4")
    (switch `/Game/Content/HUD/ShowNote/PresetShowNote` (`self.PresetNote`)
      (:`NewEnumerator0`
        (set `self.FontFamily` "/Game/Content/Font/DIEDIEDI_Font.DIEDIEDI_Font")
        (set `self.FontSize` 30)
        (set `self.PaperMaterial` "/Game/Content/HUD/Materials/M_MadPaper.M_MadPaper")
        (set `self.Color` (make `SlateColor` (struct :`R` 1.0 :`A` 1.0))))
      (:`NewEnumerator1`
        (set `self.FontFamily` "/Game/Content/Font/arsenale_white_Font.arsenale_white_Font")
        (set `self.FontSize` 40)
        (set `self.PaperMaterial` "/Game/Content/HUD/Materials/M_ChildPaper.M_ChildPaper")
        (set `self.Color` (make `SlateColor` (struct :`B` 1.0 :`A` 1.0))))
      (:`NewEnumerator2`
        (set `self.FontFamily` "/Game/Content/Font/LoversQuarrel-Regular_Font.LoversQuarrel-Regular_Font")
        (set `self.FontSize` 18)
        (set `self.PaperMaterial` "/Game/Content/HUD/Materials/M_LetterPaper.M_LetterPaper")
        (set `self.Color` (make `SlateColor` (struct :`A` 1.0))))
      (:`NewEnumerator3`
        (set `self.FontFamily` "/Game/Content/Font/Roboto-Bold_Font.Roboto-Bold_Font")
        (set `self.FontSize` 18)
        (set `self.PaperMaterial` "/Game/Content/HUD/Materials/M_WrinkledPaper.M_WrinkledPaper")
        (set `self.Color` (make `SlateColor` (struct :`R` 1.0 :`G` 1.0 :`B` 1.0 :`A` 1.0)))))))

(fn `Use Item Interact`
  (params (Item :type "/Game/Inventory/InventoryObject Object Reference"))
  (returns (Success :type Boolean))
  (return false))

(fn `UserConstructionScript`
  (`self.SetPreset`)
  (`PrimitiveComponent.SetMaterial` (`self.Plane`) 0 (`self.PaperMaterial`))
  (`SceneComponent.SetRelativeScale3D` (`self.Plane`) (`self.ScaleMesh`)))