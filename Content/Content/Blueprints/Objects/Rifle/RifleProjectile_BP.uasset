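; Rifle projectile that alerts AI perception on impact and stuns the NPC.
; At BeginPlay it caches the first NPC_BP found in the level.
; On hit it reports a damage sense event on the struck actor with the player as instigator, sends StunnedMessage to that cached NPC regardless of what was hit, then destroys itself.
; A noise-event report is present but unconnected.
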(event `self.ReceiveBeginPlay`
  (bind _outactors (`GameplayStatics.GetAllActorsOfClass` "/Game/AI/NPC_BP.NPC_BP_C"))
  (set `self.NPCReference` (`|GetArrayItem` _outactors)))

(event `self.ReceiveHit`
  (params (MyComp :type "PrimitiveComponent Object Reference") (Other :type "Actor Object Reference") (OtherComp :type "PrimitiveComponent Object Reference") (bSelfMoved :type Boolean) (HitLocation :type "Vector Structure") (HitNormal :type "Vector Structure") (NormalImpulse :type "Vector Structure") (Hit :type "HitResult Structure (by ref)"))
  (`AISense_Damage.ReportDamageEvent` Other (`GameplayStatics.GetPlayerCharacter` 0) 1.0 HitLocation HitLocation)
  (message `/Game/Content/Blueprints/BPi_Interface.Stunned` (`self.NPCReference`))
  (`self.K2_DestroyActor`))

(fn `UserConstructionScript`)