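; Rifle ammo pickup that reloads the player's rifle through an interaction.
; On interact, if the player's active inventory item is the matching weapon type and not reloaded, it marks it reloaded, refreshes inventory slots, plays a sound and destroys itself, otherwise showing a popup.
; Prompt functions pick text based on the held item, and Tick clears the custom-depth highlight when the player's trace leaves it.
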(event `self.ReceiveBeginPlay`
  (bind _asfpscharacter_bp (cast `/Game/Character/Blueprints/FPSCharacter_BP` (`GameplayStatics.GetPlayerCharacter` 0)))
  (set `self.Character` _asfpscharacter_bp))

(event `self.ReceiveTick`
  (params (DeltaSeconds :type "Float (single-precision)"))
  (bind _ammo (`self.Ammo`))
  ;[1 0 0.009008] Tick
  (if (`PrimitiveComponent.bRenderCustomDepth` _ammo)
    (if (not (== (`/Game/Character/Blueprints/FPSCharacter_BP.TraceObject` (`self.Character`)) "RifleAmmo_BP"))
      (`PrimitiveComponent.SetRenderCustomDepth` _ammo false))))

(event `/Game/Content/Blueprints/BPi_Interface.Interaction`
  (params (Interactor :type "Actor Object Reference"))
  (bind _character (`self.Character`))
  (bind _character_2 (`self.Character`))
  (bind _actualitem (`/Game/Inventory/InventoryController.ActualItem` (`/Game/Character/Blueprints/FPSCharacter_BP.InventoryControllerReference` _character_2)))
  ;[0.1567 0.7472 1] Interaction
  (if (== (`GameplayStatics.GetObjectClass` Interactor) "/Game/Character/Blueprints/FPSCharacter_BP.FPSCharacter_BP_C")
    (if (!= _actualitem null)
      (if (and (`|EnumEquality` (`/Game/Inventory/InventoryObject.Type` _actualitem) "NewEnumerator6") (not (`/Game/Inventory/InventoryObject.IsReloaded` _actualitem)))
        (set `/Game/Inventory/InventoryObject.IsReloaded` true _actualitem)
        (`/Game/Inventory/HUD/WB_Inventory.UpdateSlots` (`/Game/Character/Blueprints/FPSCharacter_BP.InventoryWpReference` _character) (`/Game/Character/Blueprints/FPSCharacter_BP.InventoryControllerReference` _character))
        (`GameplayStatics.PlaySound2D` "/Game/Content/Audio/Sounds/Spatialized/InventoryObjects/Rifle/rifleReload.rifleReload" 1.0 1.0 0.0 null null)
        (`self.K2_DestroyActor`)
        (else
          (`/Game/Inventory/HUD/WB_Inventory.PlayPopupAnimation` (`/Game/Character/Blueprints/FPSCharacter_BP.InventoryWpReference` _character_2) "You don't have your weapon or it's already reloaded !"))))))

(fn `Auto Choose Default Text WP`
  (returns (GlobalText :type Text) (SpecificText :type Text) (GlobalShow :type Boolean) (SpecificShow :type Boolean))
  (return "Take your weapon to reload" "" true false))

(fn `Auto Choose Text WP`
  (params (Item :type "/Game/Inventory/InventoryObject Object Reference"))
  (returns (GlobalText :type Text) (SpecificText :type Text) (GlobalShow :type Boolean) (SpecificShow :type Boolean))
  (if (`|EnumEquality` (`/Game/Inventory/InventoryObject.Type` Item) "NewEnumerator6")
    (return "Press F to get ammo" "" true false)
    (else
      (return "Take your weapon to reload" "" true false))))

(fn `Use Item Interact`
  (params (Item :type "/Game/Inventory/InventoryObject Object Reference"))
  (returns (Success :type Boolean))
  (return false))

(fn `UserConstructionScript`)