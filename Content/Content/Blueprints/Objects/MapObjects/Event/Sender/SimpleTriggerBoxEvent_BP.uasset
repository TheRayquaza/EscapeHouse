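; Trigger box event sender that notifies receiver map objects when an actor overlaps it.
; On overlap, it proceeds only while OneTimeSender is true and clears that flag before checking the actor, so any first overlap uses it up.
; If the actor's exact class appears in OverlappedCharacterClasses, it calls Receiver on every entry in ReceiverActorS.
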(event `self.ReceiveActorBeginOverlap`
  (params (OtherActor :type "Actor Object Reference"))
  (if (`self.OneTimeSender`)
    (set `self.OneTimeSender` false)
    (for _array_element (`self.OverlappedCharacterClasses`)
      (if (== _array_element (`GameplayStatics.GetObjectClass` OtherActor))
        (for _array_element_2 (`self.ReceiverActorS`)
          (`/Game/Content/Blueprints/Objects/MapObjects/Event/Receiver/BasicReceiver_BP.Receiver` _array_element_2))))))

(fn `UserConstructionScript`)