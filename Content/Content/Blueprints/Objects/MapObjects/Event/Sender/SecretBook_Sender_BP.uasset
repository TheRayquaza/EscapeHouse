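; Secret book map object that acts as a one-time event sender when the player interacts with it.
; Interaction clears the one-time flag and plays the Use timeline, whose Multiply track blends the actor from its initial rotation by the WantedRotation offset.
; When the timeline finishes, it calls Receiver on every linked receiver actor.
; Once the flag is false, interaction only prints a debug string.
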(event `self.ReceiveBeginPlay`
  (`parent.ReceiveBeginPlay`))

(event `/Game/Content/Blueprints/BPi_Interface.Interaction`
  (params (Interactor :type "Actor Object Reference"))
  (if (`self.OneTimeSender`)
    (set `self.OneTimeSender` false)
    (bind (_direction _multiply) (`Timeline|Use`)
      (:`Update`
        (`self.K2_SetActorRotation` (`KismetMathLibrary.MakeRotator` (+ (.roll (`self.InitialRotation`)) (* (.roll (`self.WantedRotation`)) _multiply)) (+ (.pitch (`self.InitialRotation`)) (* (.pitch (`self.WantedRotation`)) _multiply)) (+ (.yaw (`self.InitialRotation`)) (* (.yaw (`self.WantedRotation`)) _multiply)))))
      (:`Finished`
        (for _array_element (`self.ReceiverActorS`)
          (`/Game/Content/Blueprints/Objects/MapObjects/Event/Receiver/BasicReceiver_BP.Receiver` _array_element))))
    (else
      (`KismetSystemLibrary.PrintString` "Hello"))))

(fn `UserConstructionScript`
  (`parent.UserConstructionScript`))