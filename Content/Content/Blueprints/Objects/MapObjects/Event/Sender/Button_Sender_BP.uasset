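; Button sender map object that triggers linked receiver actors when interacted with.
; Interaction proceeds only while IsActivated and OneTimeSender are both true, then clears OneTimeSender so it cannot fire again and calls Receiver on every actor in ReceiverActorS.
; UseItemInteract always returns false, so using an item on the button has no effect.
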(event `/Game/Content/Blueprints/BPi_Interface.Interaction`
  (params (Interactor :type "Actor Object Reference"))
  (if (`self.IsActivated`)
    (if (`self.OneTimeSender`)
      (set `self.OneTimeSender` false)
      (for _array_element (`self.ReceiverActorS`)
        (`/Game/Content/Blueprints/Objects/MapObjects/Event/Receiver/BasicReceiver_BP.Receiver` _array_element)))))

(fn `Use Item Interact`
  (params (Item :type "/Game/Inventory/InventoryObject Object Reference"))
  (returns (Success :type Boolean))
  (return false))

(fn `UserConstructionScript`
  (`parent.UserConstructionScript`))