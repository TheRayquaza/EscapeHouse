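; A map event object, a secret book that rotates when the player interacts with it.
; It stores its starting rotation on BeginPlay.
; Interaction works only while Activated is set, clears that flag so it fires once, and plays a timeline that adds a scaled WantedRotation offset to the initial rotation.
; It rejects item-based interaction by always returning false.
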(event `self.ReceiveBeginPlay`
  (set `self.InitialRotation` (`self.K2_GetActorRotation` self)))

(event `/Game/Content/Blueprints/BPi_Interface.Interaction`
  (params (Interactor :type "Actor Object Reference"))
  (if (`self.Activated`)
    (set `self.Activated` false)
    (bind (_direction _float) (`Timeline|Animation`)
      (:`Update`
        (`self.K2_SetActorRotation` (`KismetMathLibrary.MakeRotator` (+ (.roll (`self.InitialRotation`)) (* _float (.roll (`self.WantedRotation`)))) (+ (.pitch (`self.InitialRotation`)) (* _float (.pitch (`self.WantedRotation`)))) (+ (.yaw (`self.InitialRotation`)) (* _float (.yaw (`self.WantedRotation`))))))))))

(fn `Use Item Interact`
  (params (Item :type "/Game/Inventory/InventoryObject Object Reference"))
  (returns (Success :type Boolean))
  (return false))

(fn `UserConstructionScript`)