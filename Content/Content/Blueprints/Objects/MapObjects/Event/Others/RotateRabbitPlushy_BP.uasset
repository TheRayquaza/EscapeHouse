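; Map event prop, a rabbit plushy that turns to face the player when they come close.
; It caches its actor rotation on BeginPlay and checks the player's distance every Tick.
; Within a short radius, it adds that cached rotation to the look-at rotation on all three axes and applies the sum as the mesh's relative rotation, without interpolation.
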(event `self.ReceiveBeginPlay`
  (set `self.InitialRotation` (`self.K2_GetActorRotation`)))

(event `self.ReceiveTick`
  (params (DeltaSeconds :type "Float (single-precision)"))
  (bind _returnvalue (`self.K2_GetActorLocation` (`GameplayStatics.GetPlayerCharacter` 0)))
  (bind _returnvalue_2 (`self.K2_GetActorLocation` self))
  (if (<= (`KismetMathLibrary.Vector_Distance` _returnvalue _returnvalue_2) 200.0)
    (`SceneComponent.K2_SetRelativeRotation` (`self.StaticMeshComponent`) (`KismetMathLibrary.MakeRotator` (+ (.roll (`KismetMathLibrary.FindLookAtRotation` _returnvalue_2 _returnvalue)) (.roll (`self.InitialRotation`))) (+ (.pitch (`KismetMathLibrary.FindLookAtRotation` _returnvalue_2 _returnvalue)) (.pitch (`self.InitialRotation`))) (+ (.yaw (`KismetMathLibrary.FindLookAtRotation` _returnvalue_2 _returnvalue)) (.yaw (`self.InitialRotation`)))) false false)))

(fn `UserConstructionScript`)