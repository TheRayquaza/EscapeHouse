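; Event receiver map object for a secret shelf set that rotates itself when triggered.
; BeginPlay stores the actor's starting rotation.
; Event r is gated by the OneTimeReceiver flag, which it clears before playing the Rotate timeline from the start.
; Each timeline update sets the rotation to the initial one plus WantedRotation scaled by the curve value, making the offset relative to the placed orientation.
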(event `self.ReceiveBeginPlay`
  (`parent.ReceiveBeginPlay`)
  (set `self.InitialRotation` (`self.K2_GetActorRotation` self)))

(event `self.Receiver`
  (if (`self.OneTimeReceiver`)
    (set `self.OneTimeReceiver` false)
    (bind (_direction _float) (`Timeline|Rotate` :!via `PlayFromStart`)
      (:`Update`
        (`self.K2_SetActorRotation` (`KismetMathLibrary.MakeRotator` (+ (.roll (`self.InitialRotation`)) (* (.roll (`self.WantedRotation`)) _float)) (+ (.pitch (`self.InitialRotation`)) (* (.pitch (`self.WantedRotation`)) _float)) (+ (.yaw (`self.InitialRotation`)) (* (.yaw (`self.WantedRotation`)) _float))))))))

(fn `UserConstructionScript`
  (`parent.UserConstructionScript`))