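; RockingHorse_BP is a map object that rocks continuously by animating its actor rotation.
; It stores its starting rotation on BeginPlay, and a timeline's Multiplier track scales RelativeWantedRotation as an offset added to that rotation on every update.
; Tick starts the timeline through a DoOnce that resets when the timeline finishes, so the motion repeats indefinitely.
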(event `self.ReceiveBeginPlay`
  (set `self.InitialRotation` (`self.K2_GetActorRotation`)))

(event `self.ReceiveTick`
  (params (DeltaSeconds :type "Float (single-precision)"))
  (`/Engine/EditorBlueprintResources/StandardMacros.DoOnce` false :!label _label
    (:`Completed`
      (bind (_direction _multiplier) (`Timeline|Animation` :!via `PlayFromStart`)
        (:`Update`
          (`self.K2_SetActorRotation` self (`KismetMathLibrary.MakeRotator` (+ (.roll (`self.InitialRotation`)) (* (.roll (`self.RelativeWantedRotation`)) _multiplier)) (+ (.pitch (`self.InitialRotation`)) (* (.pitch (`self.RelativeWantedRotation`)) _multiplier)) (+ (.yaw (`self.InitialRotation`)) (* (.yaw (`self.RelativeWantedRotation`)) _multiplier))) false))
        (:`Finished`
          (goto _label :!via `Reset`))))))

(fn `UserConstructionScript`)