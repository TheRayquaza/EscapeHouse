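; Interactable plank that the player can knock loose, with a configurable mesh and scale.
; Interface-style functions supply the on-screen prompts and handle item use, which plays a falling sound and reports a noise event.
; It then clears the global text, enables physics, and destroys itself after a timer, clearing the inventory selection.
; The crowbar check only feeds the return value, evaluated after IsDestroyed is set, so it does not gate removal.
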(event `self.ReceiveBeginPlay`
  ;[1 0 0] References
  (bind _asfpscharacter_bp (cast `/Game/Character/Blueprints/FPSCharacter_BP` (`GameplayStatics.GetPlayerCharacter` 0)))
  (set `self.CharacterRef` _asfpscharacter_bp)
  (`PrimitiveComponent.SetSimulatePhysics` (`self.PlankMesh`) false))

(event `DelayDestroyActor`
  ;[0 1 0.0832] Destroy Actor Event
  (`/Game/Content/HUD/WB_Interface.ShowOrHideGlobalText` (`/Game/Character/Blueprints/FPSCharacter_BP.GlobalWpReference` (`self.CharacterRef`)) false "")
  (`PrimitiveComponent.SetSimulatePhysics` (`self.PlankMesh`) true)
  (`KismetSystemLibrary.Delay` (`self.DestroyTimer`))
  (`self.K2_DestroyActor`)
  (set `/Game/Inventory/InventoryController.ActorSelected` null (`/Game/Character/Blueprints/FPSCharacter_BP.InventoryControllerReference` (`self.CharacterRef`))))

(fn `Auto Choose Default Text WP`
  (returns (GlobalText :type Text) (SpecificText :type Text) (GlobalShow :type Boolean) (SpecificShow :type Boolean))
  (return "This plank can be removed" "" true false))

(fn `Auto Choose Text WP`
  (params (Item :type "/Game/Inventory/InventoryObject Object Reference"))
  (returns (GlobalText :type Text) (SpecificText :type Text) (GlobalShow :type Boolean) (SpecificShow :type Boolean))
  (if (not (`self.IsDestroyed`))
    (return "This plank can be removed" "Press E : Destroy the plank" true true)
    (else
      (return "This plank can be removed" "" true false))))

(fn `Use Item Interact`
  (params (Item :type "/Game/Inventory/InventoryObject Object Reference"))
  (returns (Success :type Boolean))
  (bind _returnvalue (`self.K2_GetActorLocation` self))
  (set `self.IsDestroyed` true)
  (`GameplayStatics.PlaySoundAtLocation` "/Game/Content/Audio/Sounds/Spatialized/ObjectSounds/Plank/PlankFalling.PlankFalling" _returnvalue (struct) 1.0 1.0 0.0 null null null)
  (`AISense_Hearing.ReportNoiseEvent` _returnvalue 1.0 null 0.0 (`self.NoiseTag`))
  (`self.DelayDestroyActor`)
  (return (and (== (`/Game/Inventory/InventoryObject.Type` Item) 1) (not (`self.IsDestroyed`)))))

(fn `UserConstructionScript`
  (bind _mesh (`self.Mesh`))
  (`SceneComponent.SetWorldScale3D` (`self.PlankMesh`) (`self.VectorScale`))
  (if (!= _mesh null)
    (`StaticMeshComponent.SetStaticMesh` (`self.PlankMesh`) _mesh)))