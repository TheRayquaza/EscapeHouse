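; Interactable faucet object that the player toggles open and closed with an on-screen F prompt.
; Interaction flips IsOpen; opening starts the water particle and running sound and reports a small noise event at the faucet attributed to the player, while closing clears both effects.
; The construction script applies the initial open state and an optional mesh override, falling back to a default laundry sink faucet.
; Using items on it is not supported.
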(event `/Game/Content/Blueprints/BPi_Interface.Interaction`
  (params (Interactor :type "Actor Object Reference"))
  (bind _isopen (`self.IsOpen`))
  (bind _returnvalue (not _isopen))
  (if _isopen
    (set `self.IsOpen` _returnvalue)
    (`self.CloseFaucet`)
    (else
      (set `self.IsOpen` _returnvalue)
      (`self.OpenFaucet`))))

(fn `AutoChooseDefaultTextWP`
  (returns (GlobalText :type Text) (SpecificText :type Text) (GlobalShow :type Boolean) (SpecificShow :type Boolean))
  (return "Press F to open / close" "" true false))

(fn `AutoChooseTextWP`
  (params (item :type "/Game/Inventory/InventoryObject Object Reference"))
  (returns (GlobalText :type Text) (SpecificText :type Text) (GlobalShow :type Boolean) (SpecificShow :type Boolean))
  (return "Press F to open / close" "" true false))

(fn `CloseFaucet`
  (`ParticleSystemComponent.SetTemplate` (`self.P_FaucetWater1`) null)
  (`AudioComponent.Stop` (`self.FaucetOpen`)))

(fn `OpenFaucet`
  (`ParticleSystemComponent.SetTemplate` (`self.P_FaucetWater1`) "/Game/Content/Materials/SpecialMaterials/WaterFaucet/P_FaucetWater.P_FaucetWater")
  (`AudioComponent.Play` (`self.FaucetOpen`) 0.0)
  (`AISense_Hearing.ReportNoiseEvent` (`SceneComponent.K2_GetComponentLocation` (`self.StaticMeshComponent`)) 1.0 (`GameplayStatics.GetPlayerCharacter` 0) 0.0 "Little"))

(fn `Use Item Interact`
  (params (Item :type "/Game/Inventory/InventoryObject Object Reference"))
  (returns (Success :type Boolean))
  (return false))

(fn `UserConstructionScript`
  (bind _mesh (`self.Mesh`))
  (bind _staticmeshcomponent (`self.StaticMeshComponent`))
  (if (not (`self.IsOpen`))
    (`self.CloseFaucet`)
    (else
      (`self.OpenFaucet`)))
  (if (!= _mesh null)
    (`StaticMeshComponent.SetStaticMesh` _staticmeshcomponent _mesh)
    (else
      (`StaticMeshComponent.SetStaticMesh` _staticmeshcomponent "/Game/Imported/Packs/Meshes/LaundrySinkFaucet_a.LaundrySinkFaucet_a"))))