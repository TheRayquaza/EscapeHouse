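; Interactable sliding door Blueprint with a configurable mesh, defaulting to a cupboard door, that the player toggles open and closed.
; Interaction runs separate timelines that move the mesh along relative X by SlidingDoorWidth, ignoring input mid-animation.
; Each toggle plays a sound and reports a "Little" noise event instigated by the player.
; Opening derives its X from the saved Y coordinate, whereas closing uses the saved X.
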(event `/Game/Content/Blueprints/BPi_Interface.Interaction`
  (params (Interactor :type "Actor Object Reference"))
  (bind _returnvalue (`GameplayStatics.GetPlayerCharacter` 0))
  (bind _y (.y (`self.LastLocation`)))
  (bind _z (.z (`self.LastLocation`)))
  (bind _returnvalue_2 (`SceneComponent.K2_GetComponentLocation` (`self.StaticMeshComponent`)))
  (bind _staticmeshcomponent (`self.StaticMeshComponent`))
  (if (not (`self.IsAnimationPlaying`))
    (set `self.LastLocation` (`SceneComponent.RelativeLocation` _staticmeshcomponent))
    (if (not (`self.IsOpen`))
      (set `self.IsAnimationPlaying` true)
      (`AudioComponent.Play` (`self.Open`) 0.0)
      (`AISense_Hearing.ReportNoiseEvent` _returnvalue_2 1.0 _returnvalue 0.0 "Little")
      ;[1 1 1] Open
      (bind (_direction _float) (`Timeline|Timeline_0` :!via `PlayFromStart`)
        (:`Update`
          (`SceneComponent.K2_SetRelativeLocation` _staticmeshcomponent (`KismetMathLibrary.MakeVector` (- _y (* _float (`self.SlidingDoorWidth`))) _y _z) false false))
        (:`Finished`
          (set `self.IsAnimationPlaying` false :!label _label)
          (set `self.IsOpen` (not (`self.IsOpen`)))))
      (else
        (set `self.IsAnimationPlaying` true)
        (`AudioComponent.Play` (`self.Close`) 0.0)
        (`AISense_Hearing.ReportNoiseEvent` _returnvalue_2 1.0 _returnvalue 0.0 "Little")
        ;[1 1 1] Close
        (bind (_direction_2 _float_2) (`Timeline|Timeline_1` :!via `PlayFromStart`)
          (:`Update`
            (`SceneComponent.K2_SetRelativeLocation` _staticmeshcomponent (`KismetMathLibrary.MakeVector` (+ (.x (`self.LastLocation`)) (* _float_2 (`self.SlidingDoorWidth`))) _y _z) false false))
          (:`Finished`
            (goto _label)))))))

(fn `AutoChooseDefaultTextXP`
  (returns (GlobalText :type Text) (SpecificText :type Text) (GlobalShow :type Boolean) (SpecificShow :type Boolean))
  (return "Press F to open / close" "" true false))

(fn `AutoChooseTextWP`
  (params (Item :type "/Game/Inventory/InventoryObject Object Reference"))
  (returns (GlobalText :type Text) (SpecificText :type Text) (GlobalShow :type Boolean) (SpecificShow :type Boolean))
  (return "Press F to open / close" "" true false))

(fn `Use Item Interact`
  (params (Item :type "/Game/Inventory/InventoryObject Object Reference"))
  (returns (Success :type Boolean))
  (return false))

(fn `UserConstructionScript`
  (bind _staticmeshcomponent (`self.StaticMeshComponent`))
  (if (!= (`self.Mesh`) null)
    (`StaticMeshComponent.SetStaticMesh` _staticmeshcomponent (`self.Mesh`))
    (else
      (`StaticMeshComponent.SetStaticMesh` _staticmeshcomponent "/Game/Imported/Packs/Meshes/SM_Modern_Cupboard_Sliding_Door.SM_Modern_Cupboard_Sliding_Door"))))