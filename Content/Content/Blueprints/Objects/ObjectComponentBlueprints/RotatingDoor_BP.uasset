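; Interactable hinged door, by default a cupboard door mesh, that swings open or closed on interaction and shows an "F" key prompt.
; Interaction plays the Open or Close component and runs a timeline that offsets yaw from the captured rotation by DoorRotation, ignoring input mid-animation.
; CheckBug marks the door open and zeroes its rotation if the given yaw exceeds 90 degrees either way.
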(event `/Game/Content/Blueprints/BPi_Interface.Interaction`
  (params (Interactor :type "Actor Object Reference"))
  (bind _staticmeshcomponent (`self.StaticMeshComponent`))
  (if (not (`self.IsAnimationPlaying`))
    (bind _output_get (set `self.LastDoorRotation` (`SceneComponent.RelativeRotation` _staticmeshcomponent)))
    (if (not (`self.IsOpen`))
      (set `self.IsAnimationPlaying` true)
      (`AudioComponent.Play` (`self.Open`) 0.0)
      ;[1 1 1] Open
      (bind (_direction _rotation) (`Timeline|Timeline_0` :!via `PlayFromStart`)
        (:`Update`
          (bind _roll (.roll _output_get))
          (bind _pitch (.pitch _output_get))
          (bind _yaw (.yaw _output_get))
          (`SceneComponent.K2_SetRelativeRotation` _staticmeshcomponent (`KismetMathLibrary.MakeRotator` _roll _pitch (- _yaw (* _rotation (.yaw (`self.DoorRotation`))))) false false))
        (:`Finished`
          (set `self.IsAnimationPlaying` false :!label _label)
          (set `self.IsOpen` (not (`self.IsOpen`)))))
      (else
        (set `self.IsAnimationPlaying` true)
        (`AudioComponent.Play` (`self.Close`) 0.0)
        ;[1 1 1] Close
        (bind (_direction_2 _rotation_2) (`Timeline|Timeline_1` :!via `PlayFromStart`)
          (:`Update`
            (`SceneComponent.K2_SetRelativeRotation` _staticmeshcomponent (`KismetMathLibrary.MakeRotator` _roll _pitch (+ _yaw (* _rotation_2 (.yaw (`self.DoorRotation`))))) false false))
          (:`Finished`
            (goto _label)))))))

(event `Event CheckBug`
  (params (RelativeRotation :type "Rotator Structure"))
  (bind _yaw (.yaw RelativeRotation))
  (set `self.IsOpen` true)
  (if (or (< _yaw -90.0) (> _yaw 90.0))
    (`SceneComponent.K2_SetRelativeRotation` :`self` (`self.StaticMeshComponent`))))

(fn `AutoChooseDefaultTextWP`
  (returns (GlobalText :type Text) (SpecificText :type Text) (GlobalShow :type Boolean) (SpecificShow :type Boolean))
  (return "Press F to open / close" "" true false))

(fn `AutoChooseTextWP`
  (params (Item :type "/Game/Inventory/InventoryObject Object Reference"))
  (returns (GlobalText :type Text) (SpecificText :type Text) (GlobalShow :type Boolean) (SpecificShow :type Boolean))
  (return "Press F to open / close" "" true false))

(fn `Use Item Interact`
  (params (Item :type "/Game/Inventory/InventoryObject Object Reference"))
  (returns (Success :type Boolean))
  (return false))

(fn `UserConstructionScript`
  (bind _mesh (`self.Mesh`))
  (bind _staticmeshcomponent (`self.StaticMeshComponent`))
  (if (== _mesh null)
    (`StaticMeshComponent.SetStaticMesh` _staticmeshcomponent "/Game/Imported/Packs/Meshes/Fournitures_Meshes/SM_Classic_Cupboard_Door_Left.SM_Classic_Cupboard_Door_Left")
    (else
      (`StaticMeshComponent.SetStaticMesh` _staticmeshcomponent _mesh))))