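; Interactable toilet prop that the player can flush once, making noise that AI can hear.
; Interaction sets a one-way activated flag, then plays the flush sound and reports a Medium-tagged noise event at the mesh location, with the player as instigator.
; Prompt functions always show "Press F to flush", and item use on the toilet always returns false.
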(event `/Game/Content/Blueprints/BPi_Interface.Interaction`
  (params (Interactor :type "Actor Object Reference"))
  (if (not (`self.IsActivated`))
    (set `self.IsActivated` (not (`self.IsActivated`)))
    (`self.FlushActivation`)))

(event `FlushActivation`
  (`AudioComponent.Play` (`self.Flush`) 0.0)
  (`AISense_Hearing.ReportNoiseEvent` (`SceneComponent.K2_GetComponentLocation` (`self.StaticMeshComponent`)) 1.0 (`GameplayStatics.GetPlayerCharacter` 0) 0.0 "Medium"))

(fn `AutoChooseDefaultTextWP`
  (returns (GlobalText :type Text) (SpecificText :type Text) (GlobalShow :type Boolean) (SpecificShow :type Boolean))
  (return "Press F to flush" "" true false))

(fn `AutoChooseTextWP`
  (params (item :type "/Game/Inventory/InventoryObject Object Reference"))
  (returns (GlobalText :type Text) (SpecificText :type Text) (GlobalShow :type Boolean) (SpecificShow :type Boolean))
  (return "Press F to flush" "" true false))

(fn `Use Item Interact`
  (params (Item :type "/Game/Inventory/InventoryObject Object Reference"))
  (returns (Success :type Boolean))
  (return false))

(fn `UserConstructionScript`)