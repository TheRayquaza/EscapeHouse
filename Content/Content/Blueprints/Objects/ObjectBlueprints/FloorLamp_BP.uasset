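; Interactable floor lamp that the player toggles on and off through an interaction prompt.
; Interaction flips IsOn, and TurnOnOff passes it to SwitchLight on two SpecialLight child actors.
; The construction script applies that state plus configurable brightness, radius and color to both lights' point light components.
; It always shows a fixed on/off prompt, and item use returns false.
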(event `/Game/Content/Blueprints/BPi_Interface.Interaction`
  (params (Interactor :type "Actor Object Reference"))
  (set `self.IsOn` (not (`self.IsOn`)))
  (`self.TurnOnOff`))

(fn `AutoChooseDefaultTextWP`
  (returns (GlobalText :type Text) (SpecificText :type Text) (GlobalShow :type Boolean) (SpecificShow :type Boolean))
  (return "Press F to turn on / off" "" true false))

(fn `AutoChooseTextWP`
  (params (item :type "/Game/Inventory/InventoryObject Object Reference"))
  (returns (GlobalText :type Text) (SpecificText :type Text) (GlobalShow :type Boolean) (SpecificShow :type Boolean))
  (return "Press F to turn on / off" "" true false))

(fn `TurnOnOff`
  (bind _ison (`self.IsOn`))
  (bind _asspecial_light (cast `/Game/Content/Blueprints/Lights/SpecialLight` (`ChildActorComponent.ChildActor` (`self.FloorLampLight1`))))
  (bind _asspecial_light_2 (cast `/Game/Content/Blueprints/Lights/SpecialLight` (`ChildActorComponent.ChildActor` (`self.FloorLampLight2`))))
  (`/Game/Content/Blueprints/Lights/SpecialLight.SwitchLight` _asspecial_light _ison)
  (`/Game/Content/Blueprints/Lights/SpecialLight.SwitchLight` _asspecial_light_2 _ison))

(fn `Use Item Interact`
  (params (Item :type "/Game/Inventory/InventoryObject Object Reference"))
  (returns (Success :type Boolean))
  (return false))

(fn `UserConstructionScript`
  (`self.TurnOnOff`)
  (bind _asspecial_light (cast `/Game/Content/Blueprints/Lights/SpecialLight` (`ChildActorComponent.ChildActor` (`self.FloorLampLight1`))))
  (bind _pointlightcomponent (`PointLight.PointLightComponent` _asspecial_light))
  (`LightComponent.SetIntensity` _pointlightcomponent (`self.Brightness`))
  (`LocalLightComponent.SetAttenuationRadius` _pointlightcomponent (`self.Radius`))
  (`LightComponent.SetLightColor` _pointlightcomponent (`self.Color`) true)
  (bind _asspecial_light_2 (cast `/Game/Content/Blueprints/Lights/SpecialLight` (`ChildActorComponent.ChildActor` (`self.FloorLampLight2`))))
  (bind _pointlightcomponent_2 (`PointLight.PointLightComponent` _asspecial_light_2))
  (`LightComponent.SetIntensity` _pointlightcomponent_2 (`self.Brightness`))
  (`LocalLightComponent.SetAttenuationRadius` _pointlightcomponent_2 (`self.Radius`))
  (`LightComponent.SetLightColor` _pointlightcomponent_2 (`self.Color`) true))