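; Bed drawer interactive object that slides a given drawer open or closed along its local Y axis.
; OpenCloseDrawer saves the drawer mesh's relative location, plays its open or close sound, and runs a matching timeline that offsets it by CommodeWidth.
; IsAnimationPlaying blocks new requests until the timeline finishes.
; The close branch bases its new Y on the saved X, unlike the open branch.
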(event `OpenCloseDrawer`
  (params (Drawer :type "/Game/Content/Blueprints/InteractiveObjects/ObjectComponentBlueprints/Drawer_BP Object Reference") (IsClosed :type Boolean))
  (bind _staticmeshcomponent (`StaticMeshActor.StaticMeshComponent` Drawer))
  (bind _x (.x (`self.LastDrawerLocation`)))
  (bind _z (.z (`self.LastDrawerLocation`)))
  (if (not (`self.IsAnimationPlaying`))
    (set `self.LastDrawerLocation` (`SceneComponent.RelativeLocation` _staticmeshcomponent))
    (if IsClosed
      (set `self.IsAnimationPlaying` true)
      (`AudioComponent.Play` (`/Game/Content/Blueprints/InteractiveObjects/ObjectComponentBlueprints/Drawer_BP.Open` Drawer) 0.0)
      ;[1 1 1] Open
      (bind (_direction _yaxis) (`Timeline|Open` :!via `PlayFromStart`)
        (:`Update`
          (`SceneComponent.K2_SetRelativeLocation` _staticmeshcomponent (`KismetMathLibrary.MakeVector` _x (- (.y (`self.LastDrawerLocation`)) (* _yaxis (`self.CommodeWidth`))) _z) false false))
        (:`Finished`
          (set `self.IsAnimationPlaying` false :!label _label)))
      (else
        (set `self.IsAnimationPlaying` true)
        (`AudioComponent.Play` (`/Game/Content/Blueprints/InteractiveObjects/ObjectComponentBlueprints/Drawer_BP.Close` Drawer) 0.0)
        ;[1 1 1] Close
        (bind (_direction_2 _yaxis_2) (`Timeline|Close` :!via `PlayFromStart`)
          (:`Update`
            (`SceneComponent.K2_SetRelativeLocation` _staticmeshcomponent (`KismetMathLibrary.MakeVector` _x (+ _x (* _yaxis_2 (`self.CommodeWidth`))) _z) false false))
          (:`Finished`
            (goto _label)))))))

(fn `UserConstructionScript`)