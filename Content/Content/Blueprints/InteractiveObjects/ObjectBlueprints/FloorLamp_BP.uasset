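; Interactive floor lamp that the player toggles on and off, showing a "Press F to turn on / off" prompt.
; Interaction flips IsOn and calls TurnOnOff, which casts its two child-actor lights to SpecialLight and switches both to match.
; The construction script runs TurnOnOff too, so the IsOn value is applied at construction.
; Item use on the lamp always returns false.
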(event `/Game/Content/Blueprints/BPi_Interface.Interaction`
  (params (Interactor :type "Actor Object Reference"))
  (set `self.IsOn` (not (`self.IsOn`)))
  (`self.TurnOnOff`))

(fn `AutoChooseDefaultTextWP`
  (returns (GlobalText :type Text) (SpecificText :type Text) (GlobalShow :type Boolean) (SpecificShow :type Boolean))
  (return "Press F to turn on / off" "" true false))

(fn `AutoChooseTextWP`
  (params (item :type "/Game/Inventory/InventoryObject Object Reference"))
  (returns (GlobalText :type Text) (SpecificText :type Text) (GlobalShow :type Boolean) (SpecificShow :type Boolean))
  (return "Press F to turn on / off" "" true false))

(fn `TurnOnOff`
  (bind _asspecial_light (cast `/Game/Content/Blueprints/Lights/SpecialLight` (`ChildActorComponent.ChildActor` (`self.FloorLampLight1`))))
  (bind _asspecial_light_2 (cast `/Game/Content/Blueprints/Lights/SpecialLight` (`ChildActorComponent.ChildActor` (`self.FloorLampLight2`))))
  (if (`self.IsOn`)
    (`/Game/Content/Blueprints/Lights/SpecialLight.SwitchLight` _asspecial_light true)
    (`/Game/Content/Blueprints/Lights/SpecialLight.SwitchLight` _asspecial_light_2 true)
    (else
      (`/Game/Content/Blueprints/Lights/SpecialLight.SwitchLight` _asspecial_light false)
      (`/Game/Content/Blueprints/Lights/SpecialLight.SwitchLight` _asspecial_light_2 false))))

(fn `Use Item Interact`
  (params (Item :type "/Game/Inventory/InventoryObject Object Reference"))
  (returns (Success :type Boolean))
  (return false))

(fn `UserConstructionScript`
  (`self.TurnOnOff`))