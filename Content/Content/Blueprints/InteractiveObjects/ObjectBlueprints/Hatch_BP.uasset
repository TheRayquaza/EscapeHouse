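; Interactive hatch that can start padlocked and opens or closes when the player interacts with it.
; A timeline moves and rotates the hatch and tracks its state, while each use plays a sound and reports a noise event.
; An item with a matching key tag unlocks and opens it, dropping the padlock with physics before destroying it.
; The construction script sets padlock visibility and collision from the lock state, and helper functions supply prompt text.
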(event `/Game/Content/Blueprints/BPi_Interface.Interaction`
  (params (Interactor :type "Actor Object Reference"))
  (bind _returnvalue (`GameplayStatics.GetPlayerCharacter` 0))
  (bind _returnvalue_2 (`self.K2_GetActorLocation`))
  (bind _loudness (`self.Loudness`))
  (bind _noisetag (`self.NoiseTag`))
  (if (not (`self.IsLocked`))
    (switch `/Game/Content/Blueprints/Enums/DoorState` (`self.State`)
      (:`NewEnumerator0`
        ;[0.3523 0 1] Noise Event
        (`GameplayStatics.PlaySoundAtLocation` "/Game/Content/Audio/Sounds/Spatialized/ObjectSounds/Hatch/CloseHatch.CloseHatch" _returnvalue_2 (struct) 1.0 1.0 0.0 null null _returnvalue)
        (`AISense_Hearing.ReportNoiseEvent` _returnvalue_2 _loudness Interactor 0.0 _noisetag)
        ;[0 0.5302 1] Door Event
        (bind (_direction _hatchopening) (`Timeline|HatchAnimation` :!via `PlayFromStart` :!label _label)
          (:`Update`
            ;;[1 1 1] Update the rotation of the door
            (`SceneComponent.K2_SetWorldLocationAndRotation` (`self.Hatch`) (+ (`self.WorldLocation`) (* (0.0 70.0 70.0) _hatchopening)) (* (`self.OpenRotation`) _hatchopening) false false)
            (if (`|EnumEquality` _direction "Forward")
              (set `self.State` "NewEnumerator3")
              (else
                (set `self.State` "NewEnumerator2"))))
          (:`Finished`
            ;;[1 1 1] Finished Closing or Openings
            (switch `/Game/Content/Blueprints/Enums/DoorState` (`self.State`)
              (:`NewEnumerator2`
                (set `self.State` "NewEnumerator0"))
              (:`NewEnumerator3`
                (set `self.State` "NewEnumerator1"))))))
      (:`NewEnumerator1`
        (`GameplayStatics.PlaySoundAtLocation` "/Game/Content/Audio/Sounds/Spatialized/ObjectSounds/Hatch/OpenHatch.OpenHatch" _returnvalue_2 (struct) 0.5 1.0 0.0 null null _returnvalue)
        (`AISense_Hearing.ReportNoiseEvent` _returnvalue_2 _loudness Interactor 0.0 _noisetag)
        (goto _label :!via `ReverseFromEnd`))
      (:`NewEnumerator2`
        (`GameplayStatics.PlaySoundAtLocation` "/Game/Content/Audio/Sounds/Spatialized/ObjectSounds/Hatch/CloseHatch.CloseHatch" _returnvalue_2 (struct) 1.0 1.0 0.0 null null _returnvalue)
        (`AISense_Hearing.ReportNoiseEvent` _returnvalue_2 _loudness Interactor 0.0 _noisetag :!label _label_2)
        (goto _label))
      (:`NewEnumerator3`
        (`GameplayStatics.PlaySoundAtLocation` "/Game/Content/Audio/Sounds/Spatialized/ObjectSounds/Hatch/OpenHatch.OpenHatch" _returnvalue_2 (struct) 0.5 1.0 0.0 null null null)
        (goto _label_2)))))

(event `self.ReceiveBeginPlay`
  ;[1 0 0] References
  (bind _asfpscharacter_bp (cast `/Game/Character/Blueprints/FPSCharacter_BP` (`GameplayStatics.GetPlayerCharacter` 0)))
  (set `self.CharacterRef` _asfpscharacter_bp))

(event `DestroyPadlock`
  (bind _padlock (`self.Padlock`))
  ;[0 1 0.2739] Destroy Padlock
  (`PrimitiveComponent.SetSimulatePhysics` _padlock true)
  (`KismetSystemLibrary.Delay` 3.0)
  (`ActorComponent.K2_DestroyComponent` _padlock))

(fn `AutoChooseDefaultTextWP`
  (returns (GlobalText :type Text) (SpecificText :type Text) (GlobalShow :type Boolean) (SpecificShow :type Boolean))
  (if (`self.IsLocked`)
    (return "This hatch is locked" "" true false)
    (else
      (return "" "" false false))))

(fn `AutoChooseTextWP`
  (params (Item :type "/Game/Inventory/InventoryObject Object Reference"))
  (returns (GlobalText :type Text) (SpecificText :type Text) (GlobalShow :type Boolean) (SpecificShow :type Boolean))
  (if (!= Item null)
    (if (`self.IsLocked`)
      (if (== (`/Game/Inventory/InventoryObject.DoorTag` Item) (`self.KeyTag`))
        (return "The hatch is locked" "Press E : Unlock thehatch" true true)
        (else
          (return "This is not the right key" "" true false)))
      (else
        (return "" "" false false)))
    (else
      (return "" "" false false))))

(fn `Use Item Interact`
  (params (Item :type "/Game/Inventory/InventoryObject Object Reference"))
  (returns (Success :type Boolean))
  (bind _returnvalue (`self.K2_GetActorLocation`))
  (bind _returnvalue_2 (`GameplayStatics.GetPlayerCharacter` 0))
  (`KismetSystemLibrary.PrintString` "Hello")
  (if (and (== (`/Game/Inventory/InventoryObject.DoorTag` Item) (`self.KeyTag`)) (`self.IsLocked`))
    (set `self.IsLocked` false)
    (`TimelineComponent.PlayFromStart` (`self.HatchAnimation`))
    (`GameplayStatics.PlaySoundAtLocation` "/Game/Content/Audio/Sounds/Spatialized/ObjectSounds/Hatch/OpenHatch.OpenHatch" _returnvalue (struct) 1.0 1.0 0.0 null null _returnvalue_2)
    (`AISense_Hearing.ReportNoiseEvent` _returnvalue (`self.Loudness`) _returnvalue_2 0.0 (`self.NoiseTag`))
    (`self.DestroyPadlock`)
    (return true)
    (else
      (return false))))

(fn `UserConstructionScript`
  (bind _islocked (`self.IsLocked`))
  (`SceneComponent.SetVisibility` (`self.Padlock`) _islocked false)
  (if _islocked
    (`PrimitiveComponent.SetCollisionObjectType` (`self.Collider`) "ECC_WorldDynamic")
    (else
      (`PrimitiveComponent.SetCollisionObjectType` (`self.Collider`) "ECC_GameTraceChannel2")))
  (set `self.WorldLocation` (`SceneComponent.K2_GetComponentLocation` (`self.Hatch`))))