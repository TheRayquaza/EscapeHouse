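; Interactive door that can be padlocked, opened by player interaction or automatically for overlapping NPCs.
; A timeline drives rotation and an Opening/Open/Closing/Closed state, with creak sounds on movement and AI noise events on interaction or unlock.
; An item with a matching key tag unlocks and opens it, dropping the physics-simulated padlock before destroying it.
; Lock state also sets prompt texts, plus padlock visibility and collision type at construction.
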(event `/Game/Content/Blueprints/BPi_Interface.Interaction`
  (params (Interactor :type "Actor Object Reference"))
  (bind _returnvalue (`GameplayStatics.GetPlayerCharacter` 0))
  (bind _returnvalue_2 (`self.K2_GetActorLocation`))
  (bind _loudness (`self.Loudness`))
  (bind _noisetag (`self.NoiseTag`))
  (if (not (`self.IsLocked`))
    (switch `/Game/Content/Blueprints/Enums/DoorState` (`self.State`)
      (:`NewEnumerator0`
        ;[0.3523 0 1] Noise Event
        (`GameplayStatics.PlaySoundAtLocation` "/Game/Content/Audio/Sounds/Spatialized/ObjectSounds/Door/Normal/DoorCreak_Wood_Closing.DoorCreak_Wood_Closing" _returnvalue_2 (struct) 1.0 1.0 0.0 null null _returnvalue)
        (`AISense_Hearing.ReportNoiseEvent` _returnvalue_2 _loudness Interactor 0.0 _noisetag)
        ;[0 0.5302 1] Door Event
        (bind (_direction _dooropening) (`Timeline|DoorAnimation` :!via `PlayFromStart` :!label _label)
          (:`Update`
            ;;[1 1 1] Update the rotation of the door
            (`SceneComponent.K2_SetRelativeRotation` (`self.Door`) (* (`self.OpenDoorRotation`) _dooropening) false false)
            (if (`|EnumEquality` _direction "Forward")
              (set `self.State` "NewEnumerator3")
              (else
                (set `self.State` "NewEnumerator2"))))
          (:`Finished`
            ;;[1 1 1] Finished Closing or Openings
            (switch `/Game/Content/Blueprints/Enums/DoorState` (`self.State`)
              (:`NewEnumerator2`
                (set `self.State` "NewEnumerator0"))
              (:`NewEnumerator3`
                (set `self.State` "NewEnumerator1"))))))
      (:`NewEnumerator1`
        (`GameplayStatics.PlaySoundAtLocation` "/Game/Content/Audio/Sounds/Spatialized/ObjectSounds/Door/Normal/DoorCreak_Wood_Open.DoorCreak_Wood_Open" _returnvalue_2 (struct) 0.5 1.0 0.0 null null _returnvalue)
        (`AISense_Hearing.ReportNoiseEvent` _returnvalue_2 _loudness Interactor 0.0 _noisetag)
        (goto _label :!via `ReverseFromEnd`))
      (:`NewEnumerator2`
        (`GameplayStatics.PlaySoundAtLocation` "/Game/Content/Audio/Sounds/Spatialized/ObjectSounds/Door/Normal/DoorCreak_Wood_Closing.DoorCreak_Wood_Closing" _returnvalue_2 (struct) 1.0 1.0 0.0 null null _returnvalue)
        (`AISense_Hearing.ReportNoiseEvent` _returnvalue_2 _loudness Interactor 0.0 _noisetag :!label _label_2)
        (goto _label))
      (:`NewEnumerator3`
        (`GameplayStatics.PlaySoundAtLocation` "/Game/Content/Audio/Sounds/Spatialized/ObjectSounds/Door/Normal/DoorCreak_Wood_Open.DoorCreak_Wood_Open" _returnvalue_2 (struct) 0.5 1.0 0.0 null null null)
        (goto _label_2)))))

(event `self.ReceiveBeginPlay`
  ;[1 0 0] References
  (bind _asfpscharacter_bp (cast `/Game/Character/Blueprints/FPSCharacter_BP` (`GameplayStatics.GetPlayerCharacter` 0)))
  (set `self.CharacterRef` _asfpscharacter_bp))

(event `DestroyPadlock`
  (bind _padlock (`self.Padlock`))
  ;[0 1 0.2739] Destroy Padlock
  (`PrimitiveComponent.SetSimulatePhysics` _padlock true)
  (`KismetSystemLibrary.Delay` 3.0)
  (`ActorComponent.K2_DestroyComponent` _padlock))

(event `self.InteractionArea.OnComponentBeginOverlap`
  (params (OverlappedComponent :type "PrimitiveComponent Object Reference") (OtherActor :type "Actor Object Reference") (OtherComp :type "PrimitiveComponent Object Reference") (OtherBodyIndex :type Integer) (bFromSweep :type Boolean) (SweepResult :type "HitResult Structure (by ref)"))
  (bind _returnvalue (`self.K2_GetActorLocation`))
  ;[0 0.1206 1] Overlap
  ;;[1 0 0.4] NPC Overlap
  (if (and (== (`GameplayStatics.GetObjectClass` (`ActorComponent.GetOwner` (`Actor.RootComponent` OtherActor))) "/Game/AI/NPC_BP.NPC_BP_C") (not (`self.IsLocked`)))
    ;;[1 0.4 0] AI SOUND (OPENING DOOR)
    (switch `/Game/Content/Blueprints/Enums/DoorState` (`self.State`)
      (:`NewEnumerator0`
        (`GameplayStatics.PlaySoundAtLocation` "/Game/Content/Audio/Sounds/Spatialized/ObjectSounds/Door/Normal/DoorCreak_Wood_Closing.DoorCreak_Wood_Closing" _returnvalue (struct) 1.0 1.0 0.0 null null null)
        (goto _label :!via `PlayFromStart`))
      (:`NewEnumerator2`
        (`GameplayStatics.PlaySoundAtLocation` "/Game/Content/Audio/Sounds/Spatialized/ObjectSounds/Door/Normal/DoorCreak_Wood_Closing.DoorCreak_Wood_Closing" _returnvalue (struct) 1.0 1.0 0.0 null null null :!label _label_3)
        (goto _label)))))

(event `self.InteractionArea.OnComponentEndOverlap`
  (params (OverlappedComponent :type "PrimitiveComponent Object Reference") (OtherActor :type "Actor Object Reference") (OtherComp :type "PrimitiveComponent Object Reference") (OtherBodyIndex :type Integer))
  ;[0 0.1206 1] Overlap
  ;;[1 0 0.4] NPC Overlap
  (if (and (== (`GameplayStatics.GetObjectClass` (`ActorComponent.GetOwner` (`Actor.RootComponent` OtherActor))) "/Game/AI/NPC_BP.NPC_BP_C") (not (`self.IsLocked`)))
    ;;[1 0.4 0] AI SOUND (OPENING DOOR)
    (switch `/Game/Content/Blueprints/Enums/DoorState` (`self.State`)
      (:`NewEnumerator1`
        (`GameplayStatics.PlaySoundAtLocation` "/Game/Content/Audio/Sounds/Spatialized/ObjectSounds/Door/Normal/DoorCreak_Wood_Closing.DoorCreak_Wood_Closing" (`self.K2_GetActorLocation`) (struct) 1.0 1.0 0.0 null null null)
        (goto _label :!via `ReverseFromEnd`))
      (:`NewEnumerator3`
        (goto _label_3)))))

(fn `AutoChooseDefaultTextWP`
  (returns (GlobalText :type Text) (SpecificText :type Text) (GlobalShow :type Boolean) (SpecificShow :type Boolean))
  (if (`self.IsLocked`)
    (return "This door is locked" "" true false)
    (else
      (return "" "" false false))))

(fn `AutoChooseTextWP`
  (params (Item :type "/Game/Inventory/InventoryObject Object Reference"))
  (returns (GlobalText :type Text) (SpecificText :type Text) (GlobalShow :type Boolean) (SpecificShow :type Boolean))
  (if (`self.IsLocked`)
    (if (== (`/Game/Inventory/InventoryObject.DoorTag` Item) (`self.KeyTag`))
      (return "The door is locked" "Press E : Unlock the door" true true)
      (else
        (return "This is not the right key" "" true false)))
    (else
      (return "" "" false false))))

(fn `Use Item Interact`
  (params (Item :type "/Game/Inventory/InventoryObject Object Reference"))
  (returns (Success :type Boolean))
  (bind _returnvalue (`self.K2_GetActorLocation`))
  (bind _returnvalue_2 (`GameplayStatics.GetPlayerCharacter` 0))
  (if (and (== (`/Game/Inventory/InventoryObject.DoorTag` Item) (`self.KeyTag`)) (`self.IsLocked`))
    (set `self.IsLocked` false)
    (`TimelineComponent.PlayFromStart` (`self.DoorAnimation`))
    (`GameplayStatics.PlaySoundAtLocation` "/Game/Content/Audio/Sounds/Spatialized/ObjectSounds/Door/Normal/DoorCreak_Wood_Closing.DoorCreak_Wood_Closing" _returnvalue (struct) 1.0 1.0 0.0 null null _returnvalue_2)
    (`AISense_Hearing.ReportNoiseEvent` _returnvalue (`self.Loudness`) _returnvalue_2 0.0 (`self.NoiseTag`))
    (`self.DestroyPadlock`)
    (return true)
    (else
      (return false))))

(fn `UserConstructionScript`
  (bind _islocked (`self.IsLocked`))
  (`SceneComponent.SetHiddenInGame` (`self.Padlock`) (not _islocked) false)
  (if _islocked
    (`PrimitiveComponent.SetCollisionObjectType` (`self.DoorCollider`) "ECC_WorldDynamic")
    (else
      (`PrimitiveComponent.SetCollisionObjectType` (`self.DoorCollider`) "ECC_GameTraceChannel2"))))