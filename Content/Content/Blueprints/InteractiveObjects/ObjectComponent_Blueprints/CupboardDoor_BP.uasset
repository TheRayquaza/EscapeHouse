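; CupboardDoor_BP is an interactable cupboard door that works as a child actor of Classic_Cupboard_BP.
; On Interaction it asks its parent cupboard to open or close it through OpenCloseDoor, then flips its IsOpen state.
; The construction script sets the door mesh from a Mesh variable, with the left classic cupboard door as a fallback.
; It shows a global open/close prompt and its item-use check always returns false.
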(event `/Game/Content/Blueprints/BPi_Interface.Interaction`
  (params (Interactor :type "Actor Object Reference"))
  (bind _returnvalue (not (`self.IsOpen`)))
  (bind _asclassic_cupboard_bp (cast `/Game/Content/Blueprints/InteractiveObjects/Object_Blueprints/Classic_Cupboard_BP` (`self.GetAttachParentActor` self)))
  (`/Game/Content/Blueprints/InteractiveObjects/Object_Blueprints/Classic_Cupboard_BP.OpenCloseDoor` _asclassic_cupboard_bp self _returnvalue)
  (set `self.IsOpen` _returnvalue))

(fn `AutoChooseDefaultTextWP`
  (returns (GlobalText :type Text) (SpecificText :type Text) (GlobalShow :type Boolean) (SpecificShow :type Boolean))
  (return "Press F to open / close" "" true false))

(fn `AutoChooseTextWP`
  (params (Item :type "/Game/Inventory/InventoryObject Object Reference"))
  (returns (GlobalText :type Text) (SpecificText :type Text) (GlobalShow :type Boolean) (SpecificShow :type Boolean))
  (return "Press F to open / close" "" true false))

(fn `Use Item Interact`
  (params (Item :type "/Game/Inventory/InventoryObject Object Reference"))
  (returns (Success :type Boolean))
  (return false))

(fn `UserConstructionScript`
  (bind _mesh (`self.Mesh`))
  (bind _staticmeshcomponent (`self.StaticMeshComponent`))
  (if (== _mesh null)
    (`StaticMeshComponent.SetStaticMesh` _staticmeshcomponent "/Game/Imported/Packs/Meshes/Fournitures_Meshes/SM_Classic_Cupboard_Door_Left.SM_Classic_Cupboard_Door_Left")
    (else
      (`StaticMeshComponent.SetStaticMesh` _staticmeshcomponent _mesh))))