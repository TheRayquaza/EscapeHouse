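; Interactable drawer piece that attaches to a commode or bed-drawer furniture actor and opens or closes when used.
; Interaction casts the attach parent to one of three furniture Blueprints, toggles IsOpen and delegates the movement to that parent's OpenCloseDrawer.
; The construction script applies the configurable mesh, falling back to a classic commode drawer.
; The prompt functions always show the open/close text, and item use always returns false.
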(event `/Game/Content/Blueprints/BPi_Interface.Interaction`
  (params (Interactor :type "Actor Object Reference"))
  (bind _returnvalue (not (`self.IsOpen`)))
  (bind _returnvalue_2 (`self.GetAttachParentActor` self))
  (bind _asclassic_commode_bp1 (cast `/Game/Content/Blueprints/InteractiveObjects/Object_Blueprints/Classic_Commode_BP1` _returnvalue_2)
    (:`then`
      (`/Game/Content/Blueprints/InteractiveObjects/Object_Blueprints/Classic_Commode_BP1.OpenCloseDrawer` _asclassic_commode_bp1 self _returnvalue)
      (set `self.IsOpen` _returnvalue))
    (:`CastFailed`
      (bind _asclassic_commode_2_bp (cast `/Game/Content/Blueprints/InteractiveObjects/Object_Blueprints/Classic_Commode2_BP` _returnvalue_2)
        (:`then`
          (set `self.IsOpen` _returnvalue)
          (`/Game/Content/Blueprints/InteractiveObjects/Object_Blueprints/Classic_Commode2_BP.OpenCloseDrawer` _asclassic_commode_2_bp self _returnvalue))
        (:`CastFailed`
          (bind _asbed_drawer_bp (cast `/Game/Content/Blueprints/InteractiveObjects/Object_Blueprints/Bed_Drawer_BP` _returnvalue_2))
          (set `self.IsOpen` _returnvalue)
          (`/Game/Content/Blueprints/InteractiveObjects/Object_Blueprints/Bed_Drawer_BP.OpenCloseDrawer` _asbed_drawer_bp self _returnvalue))))))

(fn `Auto Choose Default Text WP`
  (returns (GlobalText :type Text) (SpecificText :type Text) (GlobalShow :type Boolean) (SpecificShow :type Boolean))
  (return "Press F to open / close" "" true false))

(fn `AutoChooseTextWP`
  (params (Item :type "/Game/Inventory/InventoryObject Object Reference"))
  (returns (GlobalText :type Text) (SpecificText :type Text) (GlobalShow :type Boolean) (SpecificShow :type Boolean))
  (return "Press F to open / close" "" true false))

(fn `Use Item Interact`
  (params (Item :type "/Game/Inventory/InventoryObject Object Reference"))
  (returns (Success :type Boolean))
  (return false))

(fn `UserConstructionScript`
  (bind _staticmeshcomponent (`self.StaticMeshComponent`))
  (bind _mesh (`self.Mesh`))
  (if (!= _mesh null)
    (`StaticMeshComponent.SetStaticMesh` _staticmeshcomponent _mesh)
    (else
      (`StaticMeshComponent.SetStaticMesh` _staticmeshcomponent "/Game/Imported/Packs/Meshes/Fournitures_Meshes/SM_Classic_Commode_Drawer_1.SM_Classic_Commode_Drawer_1"))))