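; Interactable commode drawer that slides open or closed on Interaction and shows an F-key prompt.
; Timelines offset the mesh along relative Y by CommodeWidth alongside Open/Close audio; a flag blocks input mid-slide and IsOpen flips on finish.
; The close slide builds its Y from the stored X, unlike the open slide.
; The construction script applies the chosen Mesh or a default drawer; item use returns false.
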(event `/Game/Content/Blueprints/BPi_Interface.Interaction`
  (params (Interactor :type "Actor Object Reference"))
  (bind _x (.x (`self.LastLocation`)))
  (bind _z (.z (`self.LastLocation`)))
  (bind _staticmeshcomponent (`self.StaticMeshComponent`))
  (if (not (`self.IsAnimationPlaying`))
    (set `self.LastLocation` (`SceneComponent.RelativeLocation` _staticmeshcomponent))
    (if (`self.IsOpen`)
      (set `self.IsAnimationPlaying` true)
      (`AudioComponent.Play` (`self.Open`) 0.0)
      ;[1 1 1] Open
      (bind (_direction _float) (`Timeline|OpenDrawer` :!via `PlayFromStart`)
        (:`Update`
          (`SceneComponent.K2_SetRelativeLocation` _staticmeshcomponent (`KismetMathLibrary.MakeVector` _x (- (.y (`self.LastLocation`)) (* _float (`self.CommodeWidth`))) _z) false false))
        (:`Finished`
          (set `self.IsAnimationPlaying` false :!label _label)
          (set `self.IsOpen` (not (`self.IsOpen`)))))
      (else
        (set `self.IsAnimationPlaying` true)
        (`AudioComponent.Play` (`self.Close`) 0.0)
        ;[1 1 1] Close
        (bind (_direction_2 _float_2) (`Timeline|CloseDrawer` :!via `PlayFromStart`)
          (:`Update`
            (`SceneComponent.K2_SetRelativeLocation` _staticmeshcomponent (`KismetMathLibrary.MakeVector` _x (+ _x (* _float_2 (`self.CommodeWidth`))) _z) false false))
          (:`Finished`
            (goto _label)))))))

(fn `Auto Choose Default Text WP`
  (returns (GlobalText :type Text) (SpecificText :type Text) (GlobalShow :type Boolean) (SpecificShow :type Boolean))
  (return "Press F to open / close" "" true false))

(fn `AutoChooseTextWP`
  (params (Item :type "/Game/Inventory/InventoryObject Object Reference"))
  (returns (GlobalText :type Text) (SpecificText :type Text) (GlobalShow :type Boolean) (SpecificShow :type Boolean))
  (return "Press F to open / close" "" true false))

(fn `Use Item Interact`
  (params (Item :type "/Game/Inventory/InventoryObject Object Reference"))
  (returns (Success :type Boolean))
  (return false))

(fn `UserConstructionScript`
  (bind _staticmeshcomponent (`self.StaticMeshComponent`))
  (bind _mesh (`self.Mesh`))
  (if (!= _mesh null)
    (`StaticMeshComponent.SetStaticMesh` _staticmeshcomponent _mesh)
    (else
      (`StaticMeshComponent.SetStaticMesh` _staticmeshcomponent "/Game/Imported/Packs/Meshes/Fournitures_Meshes/SM_Classic_Commode_Drawer_1.SM_Classic_Commode_Drawer_1"))))