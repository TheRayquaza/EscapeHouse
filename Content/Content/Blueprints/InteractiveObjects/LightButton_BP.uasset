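; LightButton_BP is an interactable switch that turns a set of linked BasicLights on or off together.
; Interaction flips IsOn, pushes it to each valid light via SwitchLight and plays a switch sound inside that loop, once per light.
; The Construction Script applies IsOn to the same lights, so their initial state follows the button.
; Prompt functions always show the generic press-F text, and item use always returns false.
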(event `self.ReceiveBeginPlay`
  ;[1 0 0] References
  (bind _asfpscharacter_bp (cast `/Game/Character/Blueprints/FPSCharacter_BP` (`GameplayStatics.GetPlayerCharacter` 0)))
  (set `self.CharacterRef` _asfpscharacter_bp))

(event `/Game/Content/Blueprints/BPi_Interface.Interaction`
  (params (Interactor :type "Actor Object Reference"))
  (set `self.IsOn` (not (`self.IsOn`)))
  (for _array_element (`self.BasicLights`)
    (if (!= _array_element null)
      (`/Game/Content/Blueprints/Lights/SpecialLight.SwitchLight` _array_element (`self.IsOn`))
      (`GameplayStatics.PlaySound2D` "/Game/Content/Audio/Sounds/ObjectSounds/LightButton/SwitchButton.SwitchButton" 0.75 1.0 0.0 null null))))

(fn `AutoChooseDefaultTextWP`
  (returns (GlobalText :type Text) (SpecificText :type Text) (GlobalShow :type Boolean) (SpecificShow :type Boolean))
  (return "Press F to switch on/off" "" true false))

(fn `AutoChooseTextWP`
  (params (Item :type "/Game/Inventory/InventoryObject Object Reference"))
  (returns (GlobalText :type Text) (SpecificText :type Text) (GlobalShow :type Boolean) (SpecificShow :type Boolean))
  (return "Press F to switch on/off" "" true false))

(fn `Use Item Interact`
  (params (Item :type "/Game/Inventory/InventoryObject Object Reference"))
  (returns (Success :type Boolean))
  (return false))

(fn `UserConstructionScript`
  (for _array_element (`self.BasicLights`)
    (if (!= _array_element null)
      (`/Game/Content/Blueprints/Lights/SpecialLight.SwitchLight` _array_element (`self.IsOn`)))))