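; Note_BP is an interactable paper note that shows configurable text on screen.
; The construction script applies the paper material and scale to its plane mesh.
; Interaction toggles IsNoteActive, creating a Show_Note widget styled with the note's text, font and color on activation; deactivation only clears the flag.
; Prompt functions return a fixed "Press F" hint, and UseItemInteract always returns false.
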(event `self.ReceiveBeginPlay`
  ;[1 0 0] References
  (bind _asfpscharacter_bp (cast `/Game/Character/Blueprints/FPSCharacter_BP` (`GameplayStatics.GetPlayerCharacter` 0)))
  (set `self.CharacterRef` _asfpscharacter_bp))

(event `/Game/Content/Blueprints/BPi_Interface.Interaction`
  (params (Interactor :type "Actor Object Reference"))
  ;[1 0.5 0] Interaction
  (if (`self.IsNoteActive`)
    (set `self.IsNoteActive` false)
    (else
      (set `self.IsNoteActive` true)
      (bind _returnvalue (`|CreateWidget` "/Game/Content/HUD/Show_Note.Show_Note_C"))
      (`UserWidget.AddToViewport` _returnvalue 0)
      (bind _notebody (`/Game/Content/HUD/Show_Note.NoteBody` _returnvalue))
      (`TextBlock.SetText` _notebody (`self.Note Body`))
      (`TextBlock.SetFont` _notebody (make `SlateFontInfo` (`self.FontFamily`) null (struct :`OutlineColor` (struct :`A` 1.0)) "None" (`self.FontSize`)))
      (`TextBlock.SetColorAndOpacity` _notebody (`self.Color`)))))

(fn `Auto Choose Default Text WP`
  (returns (GlobalText :type Text) (SpecificText :type Text) (GlobalShow :type Boolean) (SpecificShow :type Boolean))
  (return "Press F to see the note" "" true false))

(fn `Auto Choose Text WP`
  (params (item :type "/Game/Inventory/InventoryObject Object Reference"))
  (returns (GlobalText :type Text) (SpecificText :type Text) (GlobalShow :type Boolean) (SpecificShow :type Boolean))
  (return "Press F to see the note" "" true false))

(fn `Use Item Interact`
  (params (Item :type "/Game/Inventory/InventoryObject Object Reference"))
  (returns (Success :type Boolean))
  (return false))

(fn `UserConstructionScript`
  (`PrimitiveComponent.SetMaterial` (`self.Plane`) 0 (`self.PaperMaterial`))
  (`SceneComponent.SetRelativeScale3D` (`self.Plane`) (`self.ScaleMesh`)))