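; Interactable wardrobe the player hides in, with a prompt to press F.
; Interaction, gated by box overlap, animates the door, toggles player visibility and collision, and blends the view between player and wardrobe.
; While hidden, look input drives clamped angles that a self-recalling delayed event applies to the camera.
; Tick reads the NPC's blackboard and, if it sees the player in range, opens the door and forces the player out.
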(event `self.ReceiveBeginPlay`
  ;[1 0 0] References
  (bind _returnvalue (`GameplayStatics.GetActorOfClass` "/Game/AI/NPC_BP.NPC_BP_C"))
  (set `self.AiRef` _returnvalue)
  (bind _asfpscharacter_bp (cast `/Game/Character/Blueprints/FPSCharacter_BP` (`GameplayStatics.GetPlayerCharacter` 0)))
  (set `self.CharacterRef` _asfpscharacter_bp))

(event `/Game/Content/Blueprints/BPi_Interface.Interaction`
  (params (Interactor :type "Actor Object Reference"))
  ;[1 1 1] Hiding : get in and out of the wardrobe
  (set `/Game/Character/Blueprints/FPSCharacter_BP.IsHiding` (not (`self.IsHiding`)) (`self.CharacterRef`))
  (`/Engine/EditorBlueprintResources/StandardMacros.Gate` true :!label _label
    (:`Exit`
      (`|ExecutionSequence`
        (:`then_0`
          (`self.Hiding`)
          (`self.MoveCamera`)
          (`KismetSystemLibrary.Delay` 0.2)
          (`self.EnableInput` (`GameplayStatics.GetPlayerController` 0) :!label _label_2)
          (goto _label :!via `Open`))
        (:`then_1`
          (bind (_direction _door) (`Timeline|OpenCloseDoor` :!via `PlayFromStart`)
            (:`Update`
              (`SceneComponent.K2_SetRelativeRotation` (`self.PivotLeftDoor`) (`KismetMathLibrary.MakeRotator` 0.0 0.0 (`KismetMathLibrary.Lerp` (`self.Closed Angle`) (`self.OpenedAngle`) _door)) false false))))))))

(event `self.Box.OnComponentBeginOverlap`
  (params (OverlappedComponent :type "PrimitiveComponent Object Reference") (OtherActor :type "Actor Object Reference") (OtherComp :type "PrimitiveComponent Object Reference") (OtherBodyIndex :type Integer) (bFromSweep :type Boolean) (SweepResult :type "HitResult Structure (by ref)"))
  ;[1 1 1] Hiding : get in and out of the wardrobe
  (goto _label_2))

(event `self.Box.OnComponentEndOverlap`
  (params (OverlappedComponent :type "PrimitiveComponent Object Reference") (OtherActor :type "Actor Object Reference") (OtherComp :type "PrimitiveComponent Object Reference") (OtherBodyIndex :type Integer))
  ;[1 1 1] Hiding : get in and out of the wardrobe
  (`self.DisableInput` (`GameplayStatics.GetPlayerController` 0))
  (goto _label :!via `Close`))

(event `InputAxis|LookUp`
  (params (AxisValue :type "Float (single-precision)"))
  ;[1 1 1] Move camera while in the wardrobe
  (if (`self.IsHiding`)
    (bind _output_get (set `self.Pitch` (`KismetMathLibrary.FClamp` (+ (`self.Pitch`) AxisValue) -50.0 20.0)))
    (else
      (`Pawn.AddControllerPitchInput` (`self.CharacterRef`) AxisValue))))

(event `MoveCamera`
  ;[1 1 1] Move camera while in the wardrobe
  (if (`self.IsHiding`)
    (`SceneComponent.K2_SetRelativeRotation` (`self.Camera`) (`KismetMathLibrary.MakeRotator` 0.0 (* (stale `InputAxis|LookUp` _output_get) -1.0) (* (stale `InputAxis|Turn` _output_get) 1.0)) false false)
    (`KismetSystemLibrary.Delay` 0.001)
    (`self.MoveCamera`)))

(event `InputAxis|Turn`
  (params (AxisValue :type "Float (single-precision)"))
  ;[1 1 1] Move camera while in the wardrobe
  (if (`self.IsHiding`)
    (bind _output_get (set `self.Yaw` (`KismetMathLibrary.FClamp` (+ (`self.Yaw`) AxisValue) -60.0 60.0)))
    (else
      (`Pawn.AddControllerYawInput` (`self.CharacterRef`) AxisValue))))

(event `self.ReceiveTick`
  (params (DeltaSeconds :type "Float (single-precision)"))
  (bind _airef (`self.AiRef`))
  (bind _characterref (`self.CharacterRef`))
  ;[1 1 1] Ai catches player while he is in the Wardrobe
  ;;[1 1 1] Conditions
  (if (and (`self.IsHiding`) (`BlackboardComponent.GetValueAsBool` (`AIBlueprintHelperLibrary.GetBlackboard` _airef) "CanSeePlayer") (`BlackboardComponent.GetValueAsBool` (`AIBlueprintHelperLibrary.GetBlackboard` _airef) "IsPlayerInRange"))
    (set `self.IsHiding` false)
    (`self.DisableInput` (`GameplayStatics.GetPlayerController` 0))
    (`GameplayStatics.PlaySoundAtLocation` "/Game/Content/Audio/WardrobeSound/WardrobeOpen.WardrobeOpen" (`self.K2_GetActorLocation` self) (struct) 1.0 1.0 0.0 null null null)
    ;;[1 1 1] OpenDoorAnimation
    (bind (_direction _door) (`Timeline|OpenDoor` :!via `PlayFromStart`)
      (:`Update`
        (`SceneComponent.K2_SetRelativeRotation` (`self.PivotLeftDoor`) (`KismetMathLibrary.MakeRotator` 0.0 0.0 (`KismetMathLibrary.Lerp` (`self.Closed Angle`) (`self.OpenedAngle`) _door)) false false))
      (:`Finished`
        (`KismetSystemLibrary.Delay` 1.2)
        ;;[1 1 1] Reset camera, collision ...
        (`PlayerController.SetViewTargetWithBlend` (`GameplayStatics.GetPlayerController` 0) _characterref 0.3 "VTBlend_Linear" 0.0 false)
        (`self.SetActorHiddenInGame` _characterref false)
        (`self.SetActorEnableCollision` _characterref true)
        (bind _asfpscharacter_bp (cast `/Game/Character/Blueprints/FPSCharacter_BP` (`GameplayStatics.GetPlayerCharacter` 0))
          (:`then`
            _)
          (:`CastFailed`
            _))
        (set `/Game/Character/Blueprints/FPSCharacter_BP.IsHiding` false _asfpscharacter_bp)
        ;;[1 1 1] CloseDoorAfterThis
        (bind (_direction_2 _door_2) (`Timeline|CloseDoor` :!via `PlayFromStart`)
          (:`Update`
            (`SceneComponent.K2_SetRelativeRotation` (`self.PivotLeftDoor`) (`KismetMathLibrary.MakeRotator` 0.0 0.0 (`KismetMathLibrary.Lerp` (`self.Closed Angle`) (`self.OpenedAngle`) _door_2)) false false)))))))

(fn `Auto Choose Default Text WP`
  (returns (GlobalText :type Text) (SpecificText :type Text) (GlobalShow :type Boolean) (SpecificShow :type Boolean))
  (return "Press F to hide" "" true false))

(fn `Auto Choose Text WP`
  (params (Item :type "/Game/Inventory/InventoryObject Object Reference"))
  (returns (GlobalText :type Text) (SpecificText :type Text) (GlobalShow :type Boolean) (SpecificShow :type Boolean))
  (return "Press F to hide" "" true false))

(fn `Can Player Hide`
  (returns (Answer :type Boolean))
  (return (not (`BlackboardComponent.GetValueAsBool` (`AIBlueprintHelperLibrary.GetBlackboard` (`self.AiRef`)) "CanSeePlayer"))))

(fn `Hiding`
  (bind _returnvalue (`GameplayStatics.GetPlayerController` 0))
  (bind _characterref (`self.CharacterRef`))
  (bind _returnvalue_2 (`SceneComponent.K2_GetComponentLocation` (`self.DefaultSceneRoot`)))
  (if (`self.IsHiding`)
    (`GameplayStatics.PlaySoundAtLocation` "/Game/Content/Audio/WardrobeSound/WardrobeOpen.WardrobeOpen" _returnvalue_2 (struct) 1.0 1.0 0.0 null null null)
    (set `self.IsHiding` false)
    (`self.SetActorHiddenInGame` _characterref false)
    (`self.SetActorEnableCollision` _characterref true)
    (`PlayerController.SetViewTargetWithBlend` _returnvalue _characterref 0.8 "VTBlend_Linear" 0.0 false)
    (else
      (`GameplayStatics.PlaySoundAtLocation` "/Game/Content/Audio/WardrobeSound/WardrobeClose.WardrobeClose" _returnvalue_2 (struct) 1.0 1.0 0.0 null null null)
      (set `self.IsHiding` true)
      (`self.SetActorHiddenInGame` _characterref true)
      (`self.SetActorEnableCollision` _characterref false)
      (`PlayerController.SetViewTargetWithBlend` _returnvalue self 0.8 "VTBlend_Linear" 0.0 false)))
  (set `/Game/Character/Blueprints/FPSCharacter_BP.IsHiding` (`self.IsHiding`) (`self.CharacterRef`)))

(fn `Use Item Interact`
  (params (Item :type "/Game/Inventory/InventoryObject Object Reference"))
  (returns (Success :type Boolean))
  (return false))

(fn `UserConstructionScript`)