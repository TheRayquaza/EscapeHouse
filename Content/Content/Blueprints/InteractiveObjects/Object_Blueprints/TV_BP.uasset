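; TV_BP is an interactive antique television that the player can switch on and off.
; Interaction toggles IsOn and calls TurnOnOff, which the construction script also runs to apply the initial state.
; TurnOnOff swaps the screen material between the television image and unlit black, and starts or stops the background sound cue.
; Using an item on it always returns false.
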(event `/Game/Content/Blueprints/BPi_Interface.Interaction`
  (params (Interactor :type "Actor Object Reference"))
  (set `self.IsOn` (not (`self.IsOn`)))
  (`self.TurnOnOff`))

(fn `TurnOnOff`
  (bind _tv (`self.TV`))
  (bind _tvbackgroundsound_cue (`self.TvBackgroundSound_Cue`))
  (if (`self.IsOn`)
    (`PrimitiveComponent.SetMaterial` _tv 1 "/Game/Imported/Packs/Materials/AntiqueTelevision_b_Mat.AntiqueTelevision_b_Mat")
    (`AudioComponent.SetSound` _tvbackgroundsound_cue "/Game/Content/Audio/Sounds/ObjectSounds/TV/TvBackgroundSound_Cue.TvBackgroundSound_Cue")
    (`AudioComponent.Play` _tvbackgroundsound_cue 0.0)
    (else
      (`PrimitiveComponent.SetMaterial` _tv 1 "/Game/Imported/EF_Edie/Common/Materials/SolidColor/BlackUnlit_Mat.BlackUnlit_Mat")
      (`AudioComponent.SetSound` _tvbackgroundsound_cue null)
      (`AudioComponent.Stop` _tvbackgroundsound_cue))))

(fn `Use Item Interact`
  (params (Item :type "/Game/Inventory/InventoryObject Object Reference"))
  (returns (Success :type Boolean))
  (return false))

(fn `UserConstructionScript`
  (`self.TurnOnOff`))