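; Interactable bed the player hides under, offering a "Press F to hide" prompt.
; Interaction toggles Hiding, which switches the character's visibility and collision, blends the view between bed and player, and copies IsHiding to the character.
; Look and turn input accumulate pitch and yaw while hidden, otherwise driving the character's controller.
; MoveCamera, called on interaction, applies those values to the bed camera with clamping and inverted pitch.
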(event `self.ReceiveBeginPlay`
  ;[1 0 0] References
  (bind _asfpscharacter_bp (cast `/Game/Character/Blueprints/FPSCharacter_BP` (`GameplayStatics.GetPlayerCharacter` 0)))
  (set `self.CharacterRef` _asfpscharacter_bp))

(event `/Game/Content/Blueprints/BPi_Interface.Interaction`
  (params (Interactor :type "Actor Object Reference"))
  ;[1 0.5 0] Interact
  (`/Engine/EditorBlueprintResources/StandardMacros.Gate` true :!label _label
    (:`Exit`
      (`self.Hiding`)
      (`self.MoveCamera`)
      (`KismetSystemLibrary.Delay` 0.2)
      (`self.EnableInput` (`self.CharacterRef`) (`GameplayStatics.GetPlayerController` 0))
      (goto _label :!via `Open`))))

(event `InputAxis|LookUp`
  (params (AxisValue :type "Float (single-precision)"))
  ;[1 1 1] Move camera while under the bed
  (if (`self.IsHiding`)
    (bind _output_get (set `self.Pitch` (+ (`self.Pitch`) AxisValue)))
    (else
      (`Pawn.AddControllerPitchInput` (`self.CharacterRef`) AxisValue))))

(event `MoveCamera`
  ;[1 1 1] Move camera while under the bed
  (if (`self.IsHiding`)
    (`SceneComponent.K2_SetRelativeRotation` (`self.Camera`) (`KismetMathLibrary.MakeRotator` 0.0 (`KismetMathLibrary.FClamp` (* (stale `InputAxis|LookUp` _output_get) -1.0) -10.0 10.0) (`KismetMathLibrary.FClamp` (stale `InputAxis|Turn` _output_get) 60.0 120.0)) false false)
    (`KismetSystemLibrary.Delay` 0.001)))

(event `InputAxis|Turn`
  (params (AxisValue :type "Float (single-precision)"))
  ;[1 1 1] Move camera while under the bed
  (if (`self.IsHiding`)
    (bind _output_get (set `self.Yaw` (+ (`self.Yaw`) AxisValue)))
    (else
      (`Pawn.AddControllerYawInput` (`self.CharacterRef`) AxisValue))))

(fn `Auto Choose Default Text WP`
  (returns (GlobalText :type Text) (SpecificText :type Text) (GlobalShow :type Boolean) (SpecificShow :type Boolean))
  (return "Press F to hide" "" true false))

(fn `Auto Choose Text WP`
  (params (item :type "/Game/Inventory/InventoryObject Object Reference"))
  (returns (GlobalText :type Text) (SpecificText :type Text) (GlobalShow :type Boolean) (SpecificShow :type Boolean))
  (return "Press F to hide" "" true false))

(fn `Hiding`
  (bind _returnvalue (`GameplayStatics.GetPlayerController` 0))
  (bind _characterref (`self.CharacterRef`))
  (if (`self.IsHiding`)
    (set `self.IsHiding` false)
    (`self.SetActorHiddenInGame` _characterref false)
    (`self.SetActorEnableCollision` _characterref true)
    (`PlayerController.SetViewTargetWithBlend` _returnvalue _characterref 0.8 "VTBlend_Linear" 0.0 false)
    (else
      (set `self.IsHiding` true)
      (`self.SetActorHiddenInGame` _characterref true)
      (`self.SetActorEnableCollision` _characterref false)
      (`PlayerController.SetViewTargetWithBlend` _returnvalue self 0.8 "VTBlend_Linear" 0.0 false)))
  (bind _asfpscharacter_bp (cast `/Game/Character/Blueprints/FPSCharacter_BP` (`GameplayStatics.GetPlayerCharacter` 0)))
  (set `/Game/Character/Blueprints/FPSCharacter_BP.IsHiding` (`self.IsHiding`) _asfpscharacter_bp))

(fn `Use Item Interact`
  (params (Item :type "/Game/Inventory/InventoryObject Object Reference"))
  (returns (Success :type Boolean))
  (return false))

(fn `UserConstructionScript`)