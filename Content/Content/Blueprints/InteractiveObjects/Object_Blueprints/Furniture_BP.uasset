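; Interactable double-door furniture that the player opens and closes, with an open/close prompt.
; Interaction calls OpenDoors, where a FlipFlop sets IsOpen and plays or reverses the Opening timeline to yaw the two door pivots in opposite directions.
; Door collision is disabled during the swing and restored when the timeline finishes.
; Prompt functions return fixed text, and UseItemInteract always returns false.
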(event `self.ReceiveBeginPlay`
  ;[1 0 0] References
  (bind _asfpscharacter_bp (cast `/Game/Character/Blueprints/FPSCharacter_BP` (`GameplayStatics.GetPlayerCharacter` 0)))
  (set `self.CharacterRef` _asfpscharacter_bp))

(event `OpenDoors`
  ;[1 0 0.4295] Open Doors
  (`PrimitiveComponent.SetCollisionEnabled` (`self.Doorleft`) "NoCollision")
  (`PrimitiveComponent.SetCollisionEnabled` (`self.DoorRight`) "NoCollision")
  (`/Engine/EditorBlueprintResources/StandardMacros.FlipFlop`
    (:`A`
      (set `self.IsOpen` true)
      (bind (_direction _rotation) (`Timeline|opening` :!via `PlayFromStart` :!label _label)
        (:`Update`
          (`SceneComponent.K2_SetRelativeRotation` (`self.Pivot1`) (`KismetMathLibrary.MakeRotator` 0.0 0.0 _rotation) false false)
          (`SceneComponent.K2_SetRelativeRotation` (`self.Pivot2`) (`KismetMathLibrary.MakeRotator` 0.0 0.0 (- 0.0 _rotation)) false false))
        (:`Finished`
          (`PrimitiveComponent.SetCollisionEnabled` (`self.Doorleft`) "QueryAndPhysics")
          (`PrimitiveComponent.SetCollisionEnabled` (`self.DoorRight`) "QueryAndPhysics"))))
    (:`B`
      (set `self.IsOpen` false)
      (goto _label :!via `ReverseFromEnd`))))

(event `/Game/Content/Blueprints/BPi_Interface.Interaction`
  (params (Interactor :type "Actor Object Reference"))
  ;[1 0.5 0] Interaction
  (`self.OpenDoors`))

(fn `Auto Choose Default Text WP`
  (returns (GlobalText :type Text) (SpecificText :type Text) (GlobalShow :type Boolean) (SpecificShow :type Boolean))
  (return "Press F to open / close" "" true false))

(fn `Auto Choose Text WP`
  (params (item :type "/Game/Inventory/InventoryObject Object Reference"))
  (returns (GlobalText :type Text) (SpecificText :type Text) (GlobalShow :type Boolean) (SpecificShow :type Boolean))
  (return "Press F to open / close" "" true false))

(fn `Use Item Interact`
  (params (Item :type "/Game/Inventory/InventoryObject Object Reference"))
  (returns (Success :type Boolean))
  (return false))

(fn `UserConstructionScript`)