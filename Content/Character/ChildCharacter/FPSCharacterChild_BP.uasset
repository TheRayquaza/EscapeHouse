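; First-person player character Blueprint that handles movement, interaction and the HUD widget.
; Axis input drives look and movement with head-movement camera shake, following camera pitch when flying, while crouch toggles via FlipFlop.
; A per-tick camera sphere trace finds BPi_Interface actors, shows prompts by class name for notes, doors and drawers, and stores the target for Interact.
; Hits against NPC_BP report an AI damage event.
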(event `self.ReceiveBeginPlay`
  ;[1 0 0] References
  (bind _outactors (`GameplayStatics.GetAllActorsOfClass` "/Game/Character/Blueprints/Spawn.Spawn_C"))
  (for _array_element _outactors
    _)
  (set `self.SpawnReference` _array_element)
  (bind _returnvalue (`|CreateWidget` "/Game/Content/HUD/WB_Interface.WB_Interface_C"))
  (bind _output_get (set `self.GlobalWpReference` _returnvalue))
  (`UserWidget.AddToViewport` _output_get 0))

(event `InputAxis|LookUp`
  (params (AxisValue :type "Float (single-precision)"))
  ;[0 0.1 0.4] Base Movement
  ;;[0 1 1] Camera
  (`self.AddControllerPitchInput` AxisValue))

(event `InputAxis|MoveForward`
  (params (AxisValue :type "Float (single-precision)"))
  ;[0 0.1 0.4] Base Movement
  ;;[0 1 1] Movement
  (`self.AddMovementInput` (`KismetMathLibrary.SelectVector` (`SceneComponent.GetForwardVector` (`self.Camera`)) (`KismetMathLibrary.GetForwardVector` (`KismetMathLibrary.MakeRotator` 0.0 0.0 (.yaw (`self.GetControlRotation`)))) (`NavMovementComponent.IsFlying` (`self.CharacterMovement`))) AxisValue)
  ;;;[0 1 0.6811] Head Movement
  (`PlayerController.ClientStartCameraShake` :`self` (`GameplayStatics.GetPlayerController` 0) :`Shake` "/Game/Character/Blueprints/HeadMovement_BP.HeadMovement_BP_C" :`Scale` AxisValue))

(event `InputAxis|Turn`
  (params (AxisValue :type "Float (single-precision)"))
  ;[0 0.1 0.4] Base Movement
  ;;[0 1 1] Camera
  (`self.AddControllerYawInput` AxisValue))

(event `self.ReceiveHit`
  (params (MyComp :type "PrimitiveComponent Object Reference") (Other :type "Actor Object Reference") (OtherComp :type "PrimitiveComponent Object Reference") (bSelfMoved :type Boolean) (HitLocation :type "Vector Structure") (HitNormal :type "Vector Structure") (NormalImpulse :type "Vector Structure") (Hit :type "HitResult Structure (by ref)"))
  ;[0 0.1 0.4] Base Movement
  ;;[0 1 1] Camera
  (bind _asnpc_bp (cast `/Game/AI/NPC_BP` (`ActorComponent.GetOwner` OtherComp)))
  (`AISense_Damage.ReportDamageEvent` _asnpc_bp self 0.0 HitLocation))

(event `InputAxis|MoveRight`
  (params (AxisValue :type "Float (single-precision)"))
  ;[0 0.1 0.4] Base Movement
  ;;[0 1 1] Movement
  (`self.AddMovementInput` (`KismetMathLibrary.GetRightVector` (`KismetMathLibrary.MakeRotator` 0.0 0.0 (.yaw (`self.GetControlRotation`)))) AxisValue)
  ;;;[0 1 0.6811] Head Movement
  (`PlayerController.ClientStartCameraShake` :`self` (`GameplayStatics.GetPlayerController` 0) :`Shake` "/Game/Character/Blueprints/HeadMovement_BP.HeadMovement_BP_C" :`Scale` AxisValue))

(event `InputAction|Crouch`
  (params (Key :type "Key Structure"))
  ;[0 0.1 0.4] Base Movement
  ;;[0 1 1] Movement
  ;;;[1 1 1] Crouch
  (:`Pressed`
    (`/Engine/EditorBlueprintResources/StandardMacros.FlipFlop`
      (:`A`
        (`self.Crouch`))
      (:`B`
        (`self.UnCrouch`)))))

(event `self.ReceiveTick`
  (params (DeltaSeconds :type "Float (single-precision)"))
  (bind _globalwpreference (`self.GlobalWpReference`))
  (bind _camera (`self.Camera`))
  (bind _returnvalue (`SceneComponent.K2_GetComponentLocation` _camera))
  ;[1 1 1] Interaction
  (bind _outhit (`KismetSystemLibrary.SphereTraceSingle` _returnvalue (+ _returnvalue (* (`SceneComponent.GetForwardVector` _camera) 120.0)) 3.0 "TraceTypeQuery1"))
  (if (`KismetSystemLibrary.DoesImplementInterface` (`.HitActor` (`GameplayStatics.BreakHitResult` _outhit)) "/Game/Content/Blueprints/BPi_Interface.BPi_Interface_C")
    (set `self.LastTraceObject` (`.HitActor` (`GameplayStatics.BreakHitResult` _outhit)))
    (switch `string` (`KismetSystemLibrary.GetClassDisplayName` (`GameplayStatics.GetObjectClass` (`.HitActor` (`GameplayStatics.BreakHitResult` _outhit))))
      (:`Note_BP_C`
        (`/Game/Content/HUD/WB_Interface.ShowOrHideEverything` _globalwpreference true false "Press F to read" ""))
      (:`RotatingDoor_BP_C`
        (`/Game/Content/HUD/WB_Interface.ShowOrHideEverything` _globalwpreference true false "Press F to open/close" "" :!label _label))
      (:`SlidingDoor_BP_C`
        (goto _label))
      (:`Drawer_BP_C`
        (goto _label)))
    (else
      (set `self.LastTraceObject` null)
      (`/Game/Content/HUD/WB_Interface.ShowOrHideEverything` _globalwpreference false false "Press F to read" ""))))

(event `InputAction|Interact`
  (params (Key :type "Key Structure"))
  (bind _lasttraceobject (`self.LastTraceObject`))
  ;[1 1 1] Interaction
  (:`Pressed`
    (if (not (== _lasttraceobject null))
      (message `/Game/Content/Blueprints/BPi_Interface.Interaction` _lasttraceobject self))))

(fn `Use Item Interact`
  (params (Item :type "/Game/Inventory/InventoryObject Object Reference"))
  (returns (Success :type Boolean))
  (return false))

(fn `UserConstructionScript`)