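; World pickup actor that gives an amount of an item class to the FPS character's inventory when OnPickedUp is called.
; Sphere overlaps add and remove it from the character's PickUpActors list, which works as a queue where only the first entry shows its widget label.
; The label shows the name from the item's class defaults plus the amount.
; A partial pickup keeps the remainder; a full one reveals the next label and destroys the actor.
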(event `self.ReceiveBeginPlay`
  (`self.UpdateText`))

(event `OnPickedUp`
  (params (FPS :type "/Game/Character/Blueprints/FPSCharacter_BP Object Reference"))
  (bind _inventoryref (`/Game/Character/Blueprints/FPSCharacter_BP.InventoryRef` FPS))
  (bind _pickupactors (`/Game/Character/Blueprints/FPSCharacter_BP.PickUpActors` FPS))
  (bind _output (`|GetArrayItem` _pickupactors))
  (`/Engine/EditorBlueprintResources/StandardMacros.IsValid` _inventoryref
    (:`Is Valid`
      (bind (_success _rest) (`/Game/InventoryDeprecated/Blueprints/Inventory_BP.AddItem` _inventoryref (`self.ItemToAdd`) (`self.Amount`)))
      (if _success
        (if (> _rest 0)
          (set `self.Amount` _rest)
          (`self.UpdateText`)
          (else
            (`KismetArrayLibrary.Array_RemoveItem` _pickupactors self)
            (`/Engine/EditorBlueprintResources/StandardMacros.IsValid` _output
              (:`Is Valid`
                (`SceneComponent.SetVisibility` (`/Game/InventoryDeprecated/Blueprints/PickUp_BP.PickUpText` _output) true false)
                (`self.K2_DestroyActor`))
              (:`Is Not Valid`
                (`self.K2_DestroyActor`)))))))))

(event `self.Sphere.OnComponentBeginOverlap`
  (params (OverlappedComponent :type "PrimitiveComponent Object Reference") (OtherActor :type "Actor Object Reference") (OtherComp :type "PrimitiveComponent Object Reference") (OtherBodyIndex :type Integer) (bFromSweep :type Boolean) (SweepResult :type "HitResult Structure (by ref)"))
  (bind _asfpscharacter_bp (cast `/Game/Character/Blueprints/FPSCharacter_BP` OtherActor))
  (bind _pickupactors (`/Game/Character/Blueprints/FPSCharacter_BP.PickUpActors` _asfpscharacter_bp))
  (if (> (`KismetArrayLibrary.Array_Length` _pickupactors) 0)
    (`KismetArrayLibrary.Array_Add` _pickupactors self)
    (else
      (`SceneComponent.SetVisibility` (`self.PickUpText`) true false)
      (`KismetArrayLibrary.Array_Add` _pickupactors self))))

(event `self.Sphere.OnComponentEndOverlap`
  (params (OverlappedComponent :type "PrimitiveComponent Object Reference") (OtherActor :type "Actor Object Reference") (OtherComp :type "PrimitiveComponent Object Reference") (OtherBodyIndex :type Integer))
  (bind _asfpscharacter_bp (cast `/Game/Character/Blueprints/FPSCharacter_BP` OtherActor))
  (bind _pickupactors (`/Game/Character/Blueprints/FPSCharacter_BP.PickUpActors` _asfpscharacter_bp))
  (bind _output (`|GetArrayItem` _pickupactors))
  (if (and (`KismetSystemLibrary.IsValid` _output) (== _output self))
    (`SceneComponent.SetVisibility` (`self.PickUpText`) false false)
    (`KismetArrayLibrary.Array_RemoveItem` _pickupactors self)
    (bind _output_2 (`|GetArrayItem` (`/Game/Character/Blueprints/FPSCharacter_BP.PickUpActors` _asfpscharacter_bp)))
    (`/Engine/EditorBlueprintResources/StandardMacros.IsValid` _output_2
      (:`Is Valid`
        (`SceneComponent.SetVisibility` (`/Game/InventoryDeprecated/Blueprints/PickUp_BP.PickUpText` _output_2) true false)))
    (else
      (`KismetArrayLibrary.Array_RemoveItem` _pickupactors self))))

(fn `UpdateText`
  (bind _aspick_up_text_wp (cast `/Game/InventoryDeprecated/HUD/PickUpText_WP` (`WidgetComponent.GetUserWidgetObject` (`self.PickUpText`)))
    (:`then`
      (`TextBlock.SetText` (`/Game/InventoryDeprecated/HUD/PickUpText_WP.NameText` _aspick_up_text_wp) (`|FormatText` "{Name} ({Amount})" (`.Name_2_5C50F3334A731705874AE9B963E59539` (break `/Game/InventoryDeprecated/Structures/ItemStruct` (defaults `Object` (`self.ItemToAdd`)))) (`KismetTextLibrary.Conv_IntToText` (`self.Amount`)))))
    (:`CastFailed`
      _))
  (return))

(fn `UserConstructionScript`)